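; BP_SnapBooleProp_Box is the box-shaped variant of a snap boolean prop for level design, sized by a single Handle vector.
; Its construction script sizes the Box, takes boolean thickness from Handle X, and places two snap arrows just beyond the top and bottom faces.
; It reshapes BooleSpline into a linear rectangle in the YZ plane from Handle, then runs the parent construction script.
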(fn ConstructionScript
  (bind _handle (Variables|Default|GetHandle))
  (bind _boolespline (Variables|Default|GetBooleSpline))
  (bind _handle_2 (Variables|Default|GetHandle))
  (bind _handle_3 (Variables|Default|GetHandle))
  (bind _returnvalue (* (.z _handle_3) 1.0))
  (bind _returnvalue_2 (* (.y _handle_3) -1.0))
  (bind _returnvalue_3 (* (.y _handle_3) 1.0))
  (bind _returnvalue_4 (* (.z _handle_3) -1.0))
  (Components|Box|SetBoxExtent (Variables|Default|GetBox) _handle_2 true)
  (Variables|Default|SetBoole%20Thick (.X (Math|Vector|BreakVector _handle_2)))
  (Transformation|SetRelativeLocation (Variables|Default|GetSnapArrow) (Math|Vector|MakeVector 0.0 0.0 (* (.z _handle) 1.01)) false false)
  (Transformation|SetRelativeLocation (Variables|Default|GetSnapArrow1) (Math|Vector|MakeVector 0.0 0.0 (* (.z _handle) -1.01)) false false)
  (for _index (range 0 (- (Spline|GetNumberOfSplinePoints _boolespline) 1))
    (Spline|SetSplinePointType _boolespline _index "Linear" true)
    (Spline|SetLocationatSplinePoint (Variables|Default|GetBooleSpline) _index (Utilities|Array|Get(acopy) (Utilities|Array|MakeArray (Math|Vector|MakeVector 0.0 _returnvalue_3 _returnvalue_4) (Math|Vector|MakeVector 0.0 _returnvalue_2 _returnvalue_4) (Math|Vector|MakeVector 0.0 _returnvalue_2 _returnvalue) (Math|Vector|MakeVector 0.0 _returnvalue_3 _returnvalue)) _index) "Local" true))
  (|CallParentFunction))