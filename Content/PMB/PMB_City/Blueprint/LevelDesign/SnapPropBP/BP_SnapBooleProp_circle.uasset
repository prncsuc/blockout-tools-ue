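; Circle variant of a snappable boolean level-design prop that shapes its BooleSpline as a full circle or a half arc.
; The construction script locks Handle to the YZ plane, uses its length as the radius and places two snap arrows just beyond it on opposite sides.
; It rebuilds the spline with linear points from the generated path, chosen by the Hlaf flag, then runs the parent construction script.
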(fn ConstructionScript
  (Variables|Default|SetHandle (Math|Vector|MakeVector 0.0 (.y (Variables|Default|GetHandle)) (.z (Variables|Default|GetHandle))))
  (Transformation|SetRelativeLocation (Variables|Default|GetSnapArrow) (* (Variables|Default|GetHandle) 1.01) false false)
  (Transformation|SetRelativeLocation (Variables|Default|GetSnapArrow1) (* (Variables|Default|GetHandle) -1.01) false false)
  (Spline|ClearSplinePoints (Variables|Default|GetBooleSpline) true)
  (bind _returnvalue (Class|GeometryScriptLibraryPolyPathFunctions|CreateCirclePath3D (Math|Transform|MakeTransform "0, 0, 0" "-90.000000,0.000000,0.000000" "1.000000,1.000000,1.000000") (Math|Vector|Distance(Vector) (Variables|Default|GetHandle) "0, 0, 0") 32))
  (bind _returnvalue_2 (Class|GeometryScriptLibraryPolyPathFunctions|CreateArcPath3D (Math|Transform|MakeTransform "0, 0, 0" "-90.000000,0.000000,0.000000" "1.000000,1.000000,1.000000") (Math|Vector|Distance(Vector) (Variables|Default|GetHandle) "0, 0, 0") 32 9e+01 2.7e+02))
  (for (_array_element _array_index) (Utilities|Set|ToArray (select (Variables|Default|GetHlaf？) _returnvalue_2 _returnvalue))
    (Spline|AddSplinePoint (Variables|Default|GetBooleSpline) _array_element "Local" true)
    (Spline|SetSplinePointType (Variables|Default|GetBooleSpline) _array_index "Linear" true))
  (|CallParentFunction))