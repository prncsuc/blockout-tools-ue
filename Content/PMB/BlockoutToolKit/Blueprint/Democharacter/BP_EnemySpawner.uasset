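; BP_EnemySpawner is a one-shot trigger volume that spawns enemies when the player character enters it.
; On overlap it spawns a BP_Enemy just above each SpawnData location actor, passes that entry's patrol points as MoveToActor, then destroys itself.
; The construction script sizes and centres the box from a Handle vector.
; It also builds arrow components as a layout preview, linking box centre, spawn locations and patrol points, with random colours per patrol route.
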(event OnComponentBeginOverlap(Box)
  (params (OverlappedComponent :type Primitive%20Component%20Object%20Reference) (OtherActor :type Actor%20Object%20Reference) (OtherComp :type Primitive%20Component%20Object%20Reference) (OtherBodyIndex :type Integer) (bFromSweep :type Boolean) (SweepResult :type Hit%20Result%20Structure%20%28by%20ref%29))
  (if (== OtherActor (Game|GetPlayerCharacter 0))
    (for _array_element (Variables|Default|GetSpawnData)
      (Game|SpawnActorfromClass "/Game/PMB/BlockoutToolKit/Blueprint/Democharacter/BP_Enemy.BP_Enemy_C" (Math|Conversions|ToTransform(Vector) (+ (Transformation|GetActorLocation (.SpawnLoc (Utilities|Struct|BreakST_Actor+ActorArray _array_element))) "0.000000,0.000000,50.000000")) "AdjustIfPossibleButAlwaysSpawn" "MultiplyWithRoot" 0 (.PotrolPoint (Utilities|Struct|BreakST_Actor+ActorArray _array_element)) 0))
    (Actor|DestroyActor)))

(fn ConstructionScript
  (bind _box (Variables|Default|GetBox))
  (bind _handle (Variables|Default|GetHandle))
  (Components|Box|SetBoxExtent _box (* _handle 0.5) true)
  (Transformation|SetRelativeLocationAndRotation _box (CallFunction|ReturntoCenterPoint _handle "0, 0, 0") "0, 0, 0" false false)
  (for _array_element (Variables|Default|GetSpawnData)
    (LocalVariables|SetColor (Utilities|Struct|MakeLinearColor (Math|Random|RandomFloatinRange 0.0 1.0) (Math|Random|RandomFloatinRange 0.0 1.0) (Math|Random|RandomFloatinRange 0.0 1.0) 1.0))
    (for (_array_element_2 _array_index) (.PotrolPoint (Utilities|Struct|BreakST_Actor+ActorArray _array_element))
      (if (!= (- (Utilities|Array|Length (.PotrolPoint (Utilities|Struct|BreakST_Actor+ActorArray _array_element))) 1) _array_index)
        (CallFunction|Two-pointCreationArrow (Math|Transform|InverseTransformLocation (Transformation|GetActorTransform) (Transformation|GetActorLocation _array_element_2)) (Math|Transform|InverseTransformLocation (Transformation|GetActorTransform) (Transformation|GetActorLocation (Utilities|Array|Get(acopy) (.PotrolPoint (Utilities|Struct|BreakST_Actor+ActorArray _array_element)) (+ _array_index 1)))) (LocalVariables|GetColor) "" true "0, 0, 0" "0, 0, 0" 1.0)))
    (CallFunction|Two-pointCreationArrow (Math|Transform|InverseTransformLocation (Transformation|GetActorTransform) (Transformation|GetActorLocation (.SpawnLoc (Utilities|Struct|BreakST_Actor+ActorArray _array_element)))) (Math|Transform|InverseTransformLocation (Transformation|GetActorTransform) (Transformation|GetActorLocation (Utilities|Array|Get(acopy) (.PotrolPoint (Utilities|Struct|BreakST_Actor+ActorArray _array_element))))) (LocalVariables|GetColor) "" true "0, 0, 0" "0, 0, 0" 1.0)
    (CallFunction|Two-pointCreationArrow :Root (CallFunction|ReturntoCenterPoint "0, 0, 0" (Variables|Default|GetHandle)) :Taget (Math|Transform|InverseTransformLocation (Transformation|GetActorTransform) (Transformation|GetActorLocation (.SpawnLoc (Utilities|Struct|BreakST_Actor+ActorArray _array_element)))))))

(fn ReturntoCenterPoint
  (params (A :type Vector) (B :type Vector))
  (return (+ A (* (Math|Rotator|GetRotationXVector (Math|Rotator|FindLookatRotation A B)) (* (Math|Vector|Distance(Vector) A B) 0.5)))))

(fn Two-pointCreationArrow
  (params (Root :type Vector) (Taget :type Vector) (color :type Linear%20Color%20Structure) (Value :type Text%20%28by%20ref%29) (Open？ :type Boolean) (Offset :type Vector) (TextOffset :type Vector) (ArrowSize :type Float%20%28single-precision%29))
  ;[0 0 0] This function allows you to create an arrow component and generate text content between 2 points
  (if Open？
    (bind _returnvalue (AddComponent|AddArrowComponent false (Math|Transform|MakeTransform (+ Offset Root) (Math|Rotator|FindLookatRotation Root Taget) "1.000000,1.000000,1.000000")))
    (Components|Arrow|SetArrowColor(LinearColor) _returnvalue color)
    (Variables|/Script/Engine.ArrowComponent|SetArrowLength _returnvalue (Math|Vector|Distance(Vector) Root Taget))
    (Variables|/Script/Engine.ArrowComponent|SetArrowSize _returnvalue ArrowSize)
    (bind _returnvalue_2 (AddComponent|AddTextRenderComponent false (Math|Transform|MakeTransform (+ Taget TextOffset) (Math|Rotator|MakeRotfromY (Math|Vector|GetUnitDirection(Vector) Root Taget)) "1.000000,1.000000,1.000000")))
    (Rendering|Components|TextRender|SetText _returnvalue_2 Value)
    (Rendering|Components|TextRender|SetTextRenderColor _returnvalue_2 (Math|Conversions|ToColor(LinearColor) color))
    (Development|SetHiddeninGame _returnvalue_2 true true)
    (return _returnvalue)))