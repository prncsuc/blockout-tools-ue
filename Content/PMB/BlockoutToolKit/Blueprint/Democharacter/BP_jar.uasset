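; BP_jar is a breakable jar prop that scatters gold when broken.
; A Break event or any damage triggers it once, disabling the box collision, clearing the static mesh and enabling physics and collision damage on a Geometry Collection for the shatter.
; It spawns a random handful of Bp_Gold actors at slight horizontal offsets around itself, then destroys itself after a short delay.
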(event Custom|Break
  (bind _returnvalue (Transformation|GetActorLocation))
  (bind _geometrycollection (Variables|Default|GetGeometryCollection))
  (bind (_x _y _z) (Math|Vector|BreakVector _returnvalue))
  (if (not (Variables|Default|GetBreaked？))
    (Variables|Default|SetBreaked？ true)
    (Collision|SetCollisionEnabled (Variables|Default|GetBox) "NoCollision")
    (Class|GeometryCollectionComponent|SetEnableDamagefromCollision _geometrycollection true)
    (Collision|SetCollisionEnabled _geometrycollection "QueryAndPhysics")
    (Components|StaticMesh|SetStaticMesh (Variables|Default|Getmesh) 0)
    (for _index (range 0 (Math|Random|RandomIntegerinRange 1 5))
      (Game|SpawnActorfromClass "/Game/PMB/BlockoutToolKit/Blueprint/Democharacter/Bp_Gold.Bp_Gold_C" (Math|Transform|MakeTransform (Math|Vector|MakeVector (+ _x (Math|Random|RandomFloatinRange -3e+01 3e+01)) (+ _y (Math|Random|RandomFloatinRange -3e+01 3e+01)) _z) "0, 0, 0" "1.000000,1.000000,1.000000") "AdjustIfPossibleButAlwaysSpawn" "MultiplyWithRoot" 0 0)
      (Utilities|FlowControl|Delay 3.0)
      (Actor|DestroyActor))
    (Utilities|FlowControl|Delay 3.0)
    (Actor|DestroyActor)))

(event Game|Damage|EventAnyDamage
  (params (Damage :type Float%20%28single-precision%29) (DamageType :type Damage%20Type%20Object%20Reference) (InstigatedBy :type Controller%20Object%20Reference) (DamageCauser :type Actor%20Object%20Reference))
  (bind _returnvalue (Transformation|GetActorLocation))
  (bind _geometrycollection (Variables|Default|GetGeometryCollection))
  (bind (_x _y _z) (Math|Vector|BreakVector _returnvalue))
  (if (not (Variables|Default|GetBreaked？))
    (Variables|Default|SetBreaked？ true)
    (Collision|SetCollisionEnabled (Variables|Default|GetBox) "NoCollision")
    (Class|GeometryCollectionComponent|SetEnableDamagefromCollision _geometrycollection true)
    (Collision|SetCollisionEnabled _geometrycollection "QueryAndPhysics")
    (Components|StaticMesh|SetStaticMesh (Variables|Default|Getmesh) 0)
    (for _index (range 0 (Math|Random|RandomIntegerinRange 1 5))
      (Game|SpawnActorfromClass "/Game/PMB/BlockoutToolKit/Blueprint/Democharacter/Bp_Gold.Bp_Gold_C" (Math|Transform|MakeTransform (Math|Vector|MakeVector (+ _x (Math|Random|RandomFloatinRange -3e+01 3e+01)) (+ _y (Math|Random|RandomFloatinRange -3e+01 3e+01)) _z) "0, 0, 0" "1.000000,1.000000,1.000000") "AdjustIfPossibleButAlwaysSpawn" "MultiplyWithRoot" 0 0)
      (Utilities|FlowControl|Delay 3.0)
      (Actor|DestroyActor))
    (Utilities|FlowControl|Delay 3.0)
    (Actor|DestroyActor)))

(fn ConstructionScript)