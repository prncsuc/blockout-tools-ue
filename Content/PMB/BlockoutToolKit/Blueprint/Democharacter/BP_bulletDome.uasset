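; Projectile actor for the blockout demo character that damages whatever it hits and self-destructs after a short lifetime.
; Each Tick it moves forward by a fixed, frame-rate-dependent offset without sweeping, then sphere-traces in place against WorldStatic and Pawn objects, ignoring Negligent.
; On a hit it prints the actor's name, calls Hp on BP_Enemy, GetHit on BP_DemocharacterPMB or ApplyDamage on anything else, then destroys itself.
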(event EventBeginPlay
  (Utilities|FlowControl|Delay 3.0)
  (Actor|DestroyActor))

(event EventTick
  (params (DeltaSeconds :type Float%20%28single-precision%29))
  (bind _returnvalue (Transformation|GetActorLocation))
  (Transformation|AddActorLocalOffset "50.000000,0.000000,0.000000" false false)
  (bind (_outhit _returnvalue_2) (Collision|SphereTraceForObjects _returnvalue _returnvalue (Components|Sphere|GetScaledSphereRadius (Variables|Default|GetSphere1)) (Utilities|Array|MakeArray "ObjectTypeQuery1" "ObjectTypeQuery3") false (Utilities|Array|MakeArray (Variables|Default|Getnegligent)) "None"))
  (if _returnvalue_2
    (Development|PrintString (Utilities|GetDisplayName (.HitActor (Collision|BreakHitResult _outhit))) true false)
    (Utilities|FlowControl|Sequence
      (:then_0
        (bind _asbp_enemy (Utilities|Casting|CastToBP_Enemy (.HitActor (Collision|BreakHitResult _outhit)))
          (:then
            (Default|-Hp _asbp_enemy 1.0))
          (:CastFailed
            (bind _asbp_democharacter_pmb (Utilities|Casting|CastToBP_DemocharacterPMB (.HitActor (Collision|BreakHitResult _outhit)))
              (:then
                (Default|GetHit _asbp_democharacter_pmb))
              (:CastFailed
                (Game|Damage|ApplyDamage (.HitActor (Collision|BreakHitResult _outhit)) 1.0 0 0))))))
      (:then_1
        (Actor|DestroyActor)))))

(fn ConstructionScript)