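; Demo enemy that roams between random MoveToActor targets, shoots the player on sight and drops gold on death.
; AI Move To drives movement while a delay-based loop polls a camera-channel line trace from Sphere1 toward the player camera.
; On sight, a timeline turns it to face the player, then it spawns BP_bulletDome.
; Damage pitches Sphere1 via timeline; lethal damage blows its meshes apart with physics before destruction.
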(event Custom|-Hp
  (params (-hp :type Float%20%28double-precision%29))
  (bind _cone (Variables|Default|GetCone))
  (if (> (- (Variables|Default|GetHP) -hp) 0.0)
    (Variables|Default|SetHP (- (Variables|Default|GetHP) -hp))
    (bind _att (Timeline|-HPP PlayFromStart)
      (:Update
        (Transformation|SetRelativeRotation (Variables|Default|GetSphere1) (Math|Rotator|MakeRotator 0.0 _att 0.0) false false)))
    (else
      (Physics|SetSimulatePhysics (Variables|Default|GetSphere1) true)
      (Physics|AddRadialForce _cone (Transformation|GetWorldLocation _cone) 1e+02 1.05e+05 "RIF_Constant" false)
      (Variables|Default|SetDead true)
      (Game|SpawnActorfromClass "/Game/PMB/BlockoutToolKit/Blueprint/Democharacter/Bp_Gold.Bp_Gold_C" (Math|Conversions|ToTransform(Vector) (Transformation|GetActorLocation)) "Undefined" "MultiplyWithRoot" 0 0)
      (Utilities|FlowControl|Delay 3.0)
      (Actor|DestroyActor))))

(event EventBeginPlay
  (Audio|SpawnSoundatLocation "/Engine/VREditor/Sounds/UI/Dockable_Window_Drop.Dockable_Window_Drop" (Transformation|GetActorLocation) "0, 0, 0" 1.0 1.0 0.0 0 0)
  (Utilities|FlowControl|Delay 0.2)
  (Variables|Default|SetMove%20to (.OutItem (Utilities|Array|Random (Variables|Default|GetMove%20To%20Actor))) :!label _label)
  (AI|AIMoveTo self "0, 0, 0" (Variables|Default|GetMove%20to) 5.0 false
    (:then
      (if (CallFunction|SeePlayer?) :!label _label_2
        (Variables|Default|Setself%20Rotate (Transformation|GetActorRotation) :!label _label_3)
        (Variables|Default|SetPlayerLoc (Transformation|GetActorLocation (Game|GetPlayerCharacter 0)))
        (Variables|Default|SetFire%20ROT (Math|Rotator|FindLookatRotation (Transformation|GetActorLocation) (Variables|Default|GetPlayerLoc)))
        (bind _0_1 (Timeline|Turn%20to%20Player PlayFromStart)
          (:Update
            (Transformation|SetActorRotation (Math|Rotator|Lerp(Rotator) (Variables|Default|Getself%20Rotate) (Math|Rotator|MakeRotator 0.0 0.0 (.yaw (Math|Rotator|FindLookatRotation (Transformation|GetActorLocation) (Variables|Default|GetPlayerLoc)))) _0_1 true)))
          (:Finished
            (Game|SpawnActorfromClass "/Game/PMB/BlockoutToolKit/Blueprint/Democharacter/BP_bulletDome.BP_bulletDome_C" (Math|Transform|MakeTransform (Transformation|GetWorldLocation (Variables|Default|GetArrow1)) (Variables|Default|GetFire%20ROT) "1.000000,1.000000,1.000000") "AlwaysSpawn" "MultiplyWithRoot" 0 self 0)
            (Utilities|FlowControl|Delay 0.2)
            (if (not (Variables|Default|GetDead)) :!label _label_4
              (if (CallFunction|SeePlayer?)
                (goto _label_3)
                (else
                  (if (Math|Random|RandomBool)
                    _
                    (elif (Utilities|Array|IsValidIndex (Variables|Default|GetMove%20To%20Actor))
                      (goto _label)
                      (else
                        _)))
                  (Utilities|FlowControl|Delay 1.0)
                  (goto _label_4))))))
        (else
          (Utilities|FlowControl|Delay 0.2)
          (goto _label_2))))
    (:OnSuccess
      (goto _label_4))
    (:OnFail
      (goto _label_4))))

(event EventTick
  (params (DeltaSeconds :type Float%20%28single-precision%29)))

(fn ConstructionScript)

(fn SeePlayer?
  (bind _sphere1 (Variables|Default|GetSphere1))
  (bind _returnvalue (Transformation|GetWorldLocation _sphere1))
  (bind (_outhit _returnvalue_2) (Collision|LineTraceByChannel _returnvalue (+ _returnvalue (* (Math|Vector|GetUnitDirection(Vector) _returnvalue (Camera|GetCameraLocation (Game|GetPlayerCameraManager 0))) 2e+03)) "TraceTypeQuery2" false 0 "None"))
  (Development|PrintString (Utilities|GetDisplayName (.HitActor (Collision|BreakHitResult _outhit))) false false)
  (return (and _returnvalue_2 (== (.HitActor (Collision|BreakHitResult _outhit)) (Game|GetPlayerCharacter 0)))))