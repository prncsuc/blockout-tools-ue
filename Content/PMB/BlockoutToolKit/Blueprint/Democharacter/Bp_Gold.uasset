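; Gold pickup for the PMB demo character, built on a Cylinder mesh that animates in before it can be collected.
; After a short random delay, the Move timeline offsets it vertically with a jittered tumble, then it is righted, set Ready and spun by Rloop.
; Once Ready, player overlap or any damage grants one gold through BP_DemocharacterPMB and destroys it, including a check for a player already overlapping.
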(event OnComponentBeginOverlap(Sphere)
  (params (OverlappedComponent :type Primitive%20Component%20Object%20Reference) (OtherActor :type Actor%20Object%20Reference) (OtherComp :type Primitive%20Component%20Object%20Reference) (OtherBodyIndex :type Integer) (bFromSweep :type Boolean) (SweepResult :type Hit%20Result%20Structure%20%28by%20ref%29))
  (if (Variables|Default|GetReady)
    (bind _asbp_democharacter_pmb (Utilities|Casting|CastToBP_DemocharacterPMB OtherActor))
    (Default|AddGold _asbp_democharacter_pmb 1)
    (Actor|DestroyActor)))

(event EventBeginPlay
  (bind _returnvalue (Game|GetPlayerCharacter 0))
  (bind _cylinder (Variables|Default|GetCylinder))
  (Utilities|FlowControl|Delay (Math|Random|RandomFloatinRange 0.0 0.3))
  (Components|Timeline|SetPlayRate (Variables|Default|Getmove) 5.0)
  (bind (_direction _m _r) (Timeline|move PlayFromStart)
    (:Update
      (Transformation|SetRelativeLocation _cylinder (Math|Vector|MakeVector 0.0 0.0 _m) false false)
      (Transformation|AddLocalRotation _cylinder (Math|Rotator|MakeRotator (+ _r (Math|Random|RandomFloatinRange -5.0 5.0)) 0.0 0.0) false false))
    (:Finished
      (Utilities|FlowControl|Sequence
        (:then_0
          (bind _r_2 (Timeline|Rloop PlayFromStart)
            (:Update
              (Transformation|AddLocalRotation _cylinder (Math|Rotator|MakeRotator _r_2 0.0 0.0) false false))))
        (:then_1
          (Transformation|SetRelativeRotation _cylinder "90.000000,0.000000,0.000000" false false)
          (Variables|Default|SetReady true)
          (if (Collision|IsOverlappingActor _returnvalue :!class /Script/Engine.Actor)
            (bind _asbp_democharacter_pmb (Utilities|Casting|CastToBP_DemocharacterPMB _returnvalue))
            (Default|AddGold _asbp_democharacter_pmb 1)
            (Actor|DestroyActor)))))))

(event Game|Damage|EventAnyDamage
  (params (Damage :type Float%20%28single-precision%29) (DamageType :type Damage%20Type%20Object%20Reference) (InstigatedBy :type Controller%20Object%20Reference) (DamageCauser :type Actor%20Object%20Reference))
  (if (Variables|Default|GetReady)
    (bind _asbp_democharacter_pmb (Utilities|Casting|CastToBP_DemocharacterPMB (Game|GetPlayerCharacter 0)))
    (Default|AddGold _asbp_democharacter_pmb 1)
    (Actor|DestroyActor)))

(fn ConstructionScript)