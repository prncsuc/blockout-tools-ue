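; Blockout toolkit fence that builds a solid wall mesh along a linear spline, sized in height and thickness by a Handle.
; Construction rebuilds it with Geometry Script, extruding segment and corner polygons from offset spline points, with box-projected UVs.
; SnapCheck box-traces each segment and boolean-subtracts cutter meshes from actors snapped to the fence, which can also trigger rebuilds.
; A dynamic material instance applies optional color and texture settings.
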(event Custom|Build
  (bind _materialconfigurationarray (Variables|Default|GetMaterialConfigurationArray))
  (bind _dynamicmeshcomponent (Variables|DynamicMeshActor|GetDynamicMeshComponent))
  (Components|DestroyComponent (Actor|GetComponentsByClass "/Script/Engine.ChildActorComponent"))
  (DynamicMeshActor|ReleaseAllComputeMeshes)
  ;[0 0 0] Reset material
  (Utilities|Array|Clear (Variables|Default|GetMaterialConfigurationArray))
  (for _index (range 0 (- (Rendering|Material|GetNumMaterials _dynamicmeshcomponent) 1))
    (Rendering|Material|SetMaterial _dynamicmeshcomponent _index 0))
  (Class|DynamicMeshComponent|ValidateMaterialSlots _dynamicmeshcomponent true true)
  (bind _returnvalue (DynamicMeshActor|AllocateComputeMesh))
  (Variables|Default|SetDynmesh _returnvalue)
  (CallFunction|Buildimaster)
  (CallFunction|SnapCheck)
  (Utilities|Array|Add (Variables|Default|GetMaterialConfigurationArray) (CallFunction|CreateandSetDynamicMaterials (Variables|Default|GetMateral) (Variables|Default|GetColor%20Set) "None"))
  (Class|DynamicMeshComponent|SetDynamicMesh (Variables|DynamicMeshActor|GetDynamicMeshComponent) (Variables|Default|GetDynmesh))
  ;[0 0 0] When the material of the component is not set, it is set to the primary material
  (for (_array_element _array_index) _materialconfigurationarray
    (if (not (Utilities|IsValid _array_element))
      (Utilities|Array|SetArrayElem _materialconfigurationarray _array_index (CallFunction|CreateandSetDynamicMaterials (Variables|Default|GetMateral) (Variables|Default|GetColor%20Set) "None"))))
  (Class|DynamicMeshComponent|ConfigureMaterialSet (Variables|DynamicMeshActor|GetDynamicMeshComponent) (Variables|Default|GetMaterialConfigurationArray)))

(event EventSendUpdatedBooleanEventOfSnapPerson
  (bind _materialconfigurationarray (Variables|Default|GetMaterialConfigurationArray))
  (bind _dynamicmeshcomponent (Variables|DynamicMeshActor|GetDynamicMeshComponent))
  (Components|DestroyComponent (Actor|GetComponentsByClass "/Script/Engine.ChildActorComponent"))
  (DynamicMeshActor|ReleaseAllComputeMeshes)
  ;[0 0 0] Reset material
  (Utilities|Array|Clear (Variables|Default|GetMaterialConfigurationArray))
  (for _index (range 0 (- (Rendering|Material|GetNumMaterials _dynamicmeshcomponent) 1))
    (Rendering|Material|SetMaterial _dynamicmeshcomponent _index 0))
  (Class|DynamicMeshComponent|ValidateMaterialSlots _dynamicmeshcomponent true true)
  (bind _returnvalue (DynamicMeshActor|AllocateComputeMesh))
  (Variables|Default|SetDynmesh _returnvalue)
  (CallFunction|Buildimaster)
  (CallFunction|SnapCheck)
  (Utilities|Array|Add (Variables|Default|GetMaterialConfigurationArray) (CallFunction|CreateandSetDynamicMaterials (Variables|Default|GetMateral) (Variables|Default|GetColor%20Set) "None"))
  (Class|DynamicMeshComponent|SetDynamicMesh (Variables|DynamicMeshActor|GetDynamicMeshComponent) (Variables|Default|GetDynmesh))
  ;[0 0 0] When the material of the component is not set, it is set to the primary material
  (for (_array_element _array_index) _materialconfigurationarray
    (if (not (Utilities|IsValid _array_element))
      (Utilities|Array|SetArrayElem _materialconfigurationarray _array_index (CallFunction|CreateandSetDynamicMaterials (Variables|Default|GetMateral) (Variables|Default|GetColor%20Set) "None"))))
  (Class|DynamicMeshComponent|ConfigureMaterialSet (Variables|DynamicMeshActor|GetDynamicMeshComponent) (Variables|Default|GetMaterialConfigurationArray)))

(fn ConstructionScript
  (bind _spline (Variables|Default|GetSpline))
  (for _index (range 0 (- (Spline|GetNumberOfSplinePoints _spline) 1))
    (Spline|SetSplinePointType _spline _index "Linear" true))
  (Variables|Default|SetHandle (Math|Transform|MakeTransform (Math|Vector|MakeVector 0.0 (.y (.location (Variables|Default|GetHandle))) (.z (.location (Variables|Default|GetHandle)))) "0, 0, 0" "1.000000,1.000000,1.000000"))
  (Components|Box|SetBoxExtent (Variables|Default|GetBox) (Math|Vector|MakeVector 0.0 (.y (.location (Variables|Default|GetHandle))) (* (.z (.location (Variables|Default|GetHandle))) 0.5)) true)
  (Transformation|SetRelativeLocation (Variables|Default|GetBox) (Math|Vector|MakeVector 0.0 0.0 (* (.z (.location (Variables|Default|GetHandle))) 0.5)) false false)
  (CallFunction|Build))

(fn CreateandSetDynamicMaterials
  (params (Materal :type Material%20Interface%20Object%20Reference) (ColorSet :type ST%20Color%20Set%20V2%20Structure) (OptionalName :type Name))
  (bind (_enableset _texture _normaltex _hue _saturation _light _rough _coloroverlay _tlie _rotate) (Utilities|Struct|BreakST_ColorSetV2 ColorSet))
  (bind _returnvalue (Rendering|Material|CreateDynamicMaterialInstance (Variables|DynamicMeshActor|GetDynamicMeshComponent) (Utilities|Array|Length (Variables|Default|GetMaterialConfigurationArray)) (select (Utilities|IsValid Materal) Materal "/Game/PMB/BlockoutToolKit/Materials/Adjustable/MI_PMB_Adj__cement.MI_PMB_Adj__cement") OptionalName :!class /Script/Engine.PrimitiveComponent))
  (if _enableset
    (Rendering|Material|SetVectorParameterValue _returnvalue "Color" (Utilities|Struct|MakeLinearColor _hue _saturation _light _rough) :!class /Script/Engine.MaterialInstanceDynamic)
    (Rendering|Material|SetTextureParameterValue _returnvalue "Texture" _texture)
    (Rendering|Material|SetTextureParameterValue _returnvalue "Normal" _normaltex)
    (Rendering|Material|SetScalarParameterValue _returnvalue "Tlie" (Math|Conversions|ToFloat(Integer) _tlie) :!class /Script/Engine.MaterialInstanceDynamic)
    (Rendering|Material|SetScalarParameterValue _returnvalue "rotate" (Math|Float|MapRangeClamped (Math|Conversions|ToFloat(Integer) _rotate) 0.0 3.6e+02 0.0 1.0) :!class /Script/Engine.MaterialInstanceDynamic)
    (Rendering|Material|SetVectorParameterValue _returnvalue "ColorOverlay" _coloroverlay :!class /Script/Engine.MaterialInstanceDynamic))
  (return _returnvalue))

(fn GetNextSplinePoint
  (params (Current%20index :type Integer) (next？ :type Boolean))
  (bind _returnvalue (+ Current%20index 1))
  (if next？
    (return (select (== _returnvalue (Spline|GetNumberOfSplinePoints (Variables|Default|GetSpline))) 0 _returnvalue))
    (else
      (return (select (== Current%20index 0) (- (Spline|GetNumberOfSplinePoints (Variables|Default|GetSpline)) 1) (- Current%20index 1))))))

(fn GetSplinePointMidDirectionRight
  (params (Spline :type Spline%20Component%20Object%20Reference) (PointIndex :type Integer))
  (bind _returnvalue (Spline|GetLocationatSplinePoint Spline PointIndex "Local"))
  (bind _index (CallFunction|GetNextSplinePoint PointIndex false))
  (bind _index_2 (CallFunction|GetNextSplinePoint PointIndex true))
  (bind _returnvalue_2 (Spline|GetNumberOfSplinePoints Spline))
  (bind _returnvalue_3 (Spline|GetLocationatSplinePoint Spline _index_2 "Local"))
  (bind _returnvalue_4 (Spline|GetLocationatSplinePoint Spline _index "Local"))
  (bind _returnvalue_5 (- _returnvalue_2 1))
  (bind _returnvalue_6 (Math|Vector|GetUnitDirection(Vector) _returnvalue_3 _returnvalue))
  (bind _returnvalue_7 (Math|Vector|GetUnitDirection(Vector) _returnvalue _returnvalue_4))
  (bind _returnvalue_8 (Math|Conversions|ToVector2D(Vector) _returnvalue_7))
  (bind _returnvalue_9 (Math|Conversions|ToVector2D(Vector) _returnvalue_6))
  (bind _returnvalue_10 (Class|KismetMathLibrary|CrossProduct2D _returnvalue_8 _returnvalue_9))
  (bind _returnvalue_11 (> _returnvalue_10 0.0))
  (return (select (== PointIndex 0) (Class|SplineComponent|GetRightVectoratSplinePoint Spline 0 "Local") (select (== PointIndex _returnvalue_5) (Class|SplineComponent|GetRightVectoratSplinePoint Spline _returnvalue_5 "Local") (Math|Vector|Normalize (* (+ (Math|Vector|GetUnitDirection(Vector) _returnvalue _returnvalue_4) (Math|Vector|GetUnitDirection(Vector) _returnvalue _returnvalue_3)) (select _returnvalue_11 1.0 -1.0))))) _returnvalue_11))

(fn GetRetractPointPositionandRotation
  (params (PointIndex :type Integer) (retract :type Float%20%28double-precision%29) (spline :type Spline%20Component%20Object%20Reference))
  (bind _spline (LocalVariables|GetSpline))
  (bind _right_direction (CallFunction|GetSplinePointMidDirectionRight _spline PointIndex))
  (return (+ (* _right_direction (/ retract (Math|Trig|Cos(Degrees) (* (- 1.8e+02 (CallFunction|GetSplinePointHorizontalAngle PointIndex spline)) 0.5)))) (Spline|GetLocationatSplinePoint spline PointIndex "Local")) (Class|KismetMathLibrary|MakeRotfromYZ _right_direction (Math|Vector|MakeVector 0.0 0.0 1.0))))

(fn GetSplinePointArray
  (params (Spline :type Spline%20Component%20Object%20Reference) (CoordinateSpace :type ESplineCoordinateSpace%20Enum :default "Local") (retract :type Float%20%28double-precision%29) (ZOffset :type Float%20%28double-precision%29))
  (for _index (range 0 (- (Spline|GetNumberOfSplinePoints Spline) 1))
    (Development|PrintString (Utilities|String|ToString(Vector) (.Location (CallFunction|GetRetractPointPositionandRotation _index retract Spline))) false false)
    (Utilities|Array|Add (LocalVariables|GetPointRef) (Math|Transform|MakeTransform (+ (.Location (CallFunction|GetRetractPointPositionandRotation _index retract Spline)) (* (Math|Vector|GetUpVector (.Rotation (Math|Transform|BreakTransform (Spline|GetTransformatSplinePoint Spline _index CoordinateSpace false)))) ZOffset)) (.Rotation (CallFunction|GetRetractPointPositionandRotation _index retract Spline)) (.Scale (Math|Transform|BreakTransform (Spline|GetTransformatSplinePoint Spline _index CoordinateSpace false)))))
    (Utilities|Array|Add (LocalVariables|GetPointR) (+ (.Location (CallFunction|GetRetractPointPositionandRotation _index retract Spline)) (* (Math|Vector|GetUpVector (.Rotation (Math|Transform|BreakTransform (Spline|GetTransformatSplinePoint Spline _index CoordinateSpace false)))) ZOffset))))
  (return (LocalVariables|GetPointR) (LocalVariables|GetPointRef)))

(fn Create2DRecOffset
  (params (size :type Vector%202D%20Structure) (Offset2D+Rotator :type Vector))
  (bind (_x _y) (Math|Vector2D|BreakVector2D size))
  (bind _returnvalue (* _x -0.5))
  (bind _returnvalue_2 (* _y -0.5))
  (bind _returnvalue_3 (* _x 0.5))
  (bind _returnvalue_4 (* _y 0.5))
  (LocalVariables|SetOffset Offset2D+Rotator)
  (for _array_element (Utilities|Array|MakeArray (Math|Vector2D|MakeVector2D _returnvalue_3 _returnvalue_4) (Math|Vector2D|MakeVector2D _returnvalue _returnvalue_4) (Math|Vector2D|MakeVector2D _returnvalue _returnvalue_2) (Math|Vector2D|MakeVector2D _returnvalue_3 _returnvalue_2))
    (Utilities|Array|Add (LocalVariables|Getcollect1) (+ _array_element (Math|Vector2D|MakeVector2D (.x (LocalVariables|GetOffset)) (.y (LocalVariables|GetOffset))))))
  (for _array_element_2 (LocalVariables|Getcollect1)
    (Utilities|Array|Add (LocalVariables|Getcollect2) (Math|Conversions|ToVector2D(Vector) (+ (* (Math|Vector|RotateVectorAroundAxis (Math|Vector|GetUnitDirection(Vector) (Math|Conversions|ToVector(Vector2D) (Math|Vector2D|MakeVector2D (.x (LocalVariables|GetOffset)) (.y (LocalVariables|GetOffset)))) (Math|Conversions|ToVector(Vector2D) _array_element_2)) (.z (LocalVariables|GetOffset)) "0.000000,0.000000,1.000000") (Math|Vector|Distance(Vector) (Math|Conversions|ToVector(Vector2D) _array_element_2) (Math|Conversions|ToVector(Vector2D) (Math|Vector2D|MakeVector2D (.x (LocalVariables|GetOffset)) (.y (LocalVariables|GetOffset)))))) (Math|Conversions|ToVector(Vector2D) (Math|Vector2D|MakeVector2D (.x (LocalVariables|GetOffset)) (.y (LocalVariables|GetOffset))))))))
  (return (LocalVariables|Getcollect2)))

(fn Buildimaster
  (bind _returnvalue (Transformation|GetActorTransform))
  (bind _spline (Variables|Default|GetSpline))
  (bind _spline_2 (Variables|Default|GetSpline))
  (bind _mat_world_align_ (Variables|Default|GetMat%20World%20Align?))
  (bind _returnvalue_2 (Spline|GetTransformatSplinePoint _spline 0 "Local" false))
  (bind _returnvalue_3 (Spline|GetNumberOfSplinePoints _spline_2))
  (bind _returnvalue_4 (- _returnvalue_3 1))
  (bind _returnvalue_5 (Spline|GetTransformatSplinePoint _spline_2 _returnvalue_4 "Local" false))
  (LocalVariables|SetHandleLoc (.location (Variables|Default|GetHandle)))
  (LocalVariables|SetThickRef (* (Math|Vector|Distance2D(Vector) (LocalVariables|GetHandleLoc) "0, 0, 0") 2.0))
  (LocalVariables|SetRightMidRef (.Re (CallFunction|GetSplinePointArray (Variables|Default|GetSpline) "Local" (* (LocalVariables|GetThickRef) 0.5) 0.0)))
  (LocalVariables|SetLeftMidRef (.Re (CallFunction|GetSplinePointArray (Variables|Default|GetSpline) "Local" (* (* (LocalVariables|GetThickRef) 0.5) -1.0) 0.0)))
  (for _index (range 0 (- (Spline|GetNumberOfSplinePoints (Variables|Default|GetSpline)) 2))
    (LocalVariables|SetIndexRef _index)
    (LocalVariables|SetNextIndexRef (+ _index 1))
    (Utilities|Array|Add (LocalVariables|GetAllWallPoint) (Utilities|Struct|MakeST_VectorArray (Utilities|Array|MakeArray (select (== (LocalVariables|GetIndexRef) 0) (+ (.location _returnvalue_2) (* (* (Math|Vector|GetRightVector (.rotation _returnvalue_2)) (LocalVariables|GetThickRef) 0.5) -1.0)) (select (.Is%20Turn%20Right? (CallFunction|GetSplinePointMidDirectionRight (Variables|Default|GetSpline) (LocalVariables|GetIndexRef))) (+ (Utilities|Array|Get(acopy) (LocalVariables|GetRightMidRef) (LocalVariables|GetIndexRef)) (* (Math|Vector|GetRightVector (Spline|GetRotationatSplinePoint (Variables|Default|GetSpline) (LocalVariables|GetIndexRef) "Local")) (LocalVariables|GetThickRef) -1.0)) (Utilities|Array|Get(acopy) (LocalVariables|GetLeftMidRef) (LocalVariables|GetIndexRef)))) (select (== (LocalVariables|GetIndexRef) 0) (+ (.location _returnvalue_2) (* (Math|Vector|GetRightVector (.rotation _returnvalue_2)) (LocalVariables|GetThickRef) 0.5)) (select (.Is%20Turn%20Right? (CallFunction|GetSplinePointMidDirectionRight (Variables|Default|GetSpline) (LocalVariables|GetIndexRef))) (Utilities|Array|Get(acopy) (LocalVariables|GetRightMidRef) (LocalVariables|GetIndexRef)) (+ (Utilities|Array|Get(acopy) (LocalVariables|GetLeftMidRef) (LocalVariables|GetIndexRef)) (* (Math|Vector|GetRightVector (Spline|GetRotationatSplinePoint (Variables|Default|GetSpline) (LocalVariables|GetIndexRef) "Local")) (LocalVariables|GetThickRef))))) (select (== (LocalVariables|GetIndexRef) (- (Spline|GetNumberOfSplinePoints (Variables|Default|GetSpline)) 2)) (+ (* (Math|Vector|GetRightVector (.rotation _returnvalue_5)) (LocalVariables|GetThickRef) 0.5) (.location _returnvalue_5)) (select (.Is%20Turn%20Right? (CallFunction|GetSplinePointMidDirectionRight (Variables|Default|GetSpline) (+ (LocalVariables|GetIndexRef) 1))) (Utilities|Array|Get(acopy) (LocalVariables|GetRightMidRef) (+ (LocalVariables|GetIndexRef) 1)) (+ (Utilities|Array|Get(acopy) (LocalVariables|GetLeftMidRef) (+ (LocalVariables|GetIndexRef) 1)) (* (Math|Vector|GetRightVector (Spline|GetRotationatSplinePoint (Variables|Default|GetSpline) (LocalVariables|GetIndexRef) "Local")) (LocalVariables|GetThickRef))))) (select (== (LocalVariables|GetIndexRef) (- (Spline|GetNumberOfSplinePoints (Variables|Default|GetSpline)) 2)) (+ (.location _returnvalue_5) (* (* (Math|Vector|GetRightVector (.rotation _returnvalue_5)) (LocalVariables|GetThickRef) 0.5) -1.0)) (select (.Is%20Turn%20Right? (CallFunction|GetSplinePointMidDirectionRight (Variables|Default|GetSpline) (+ (LocalVariables|GetIndexRef) 1))) (+ (Utilities|Array|Get(acopy) (LocalVariables|GetRightMidRef) (+ (LocalVariables|GetIndexRef) 1)) (* (Math|Vector|GetRightVector (Spline|GetRotationatSplinePoint (Variables|Default|GetSpline) (LocalVariables|GetIndexRef) "Local")) (LocalVariables|GetThickRef) -1.0)) (Utilities|Array|Get(acopy) (LocalVariables|GetLeftMidRef) (+ (LocalVariables|GetIndexRef) 1)))))))
    (if (!= _index (- (Spline|GetNumberOfSplinePoints (Variables|Default|GetSpline)) 2))
      (Utilities|Array|Add (LocalVariables|GetAll%20corner%20Point) (Utilities|Struct|MakeST_VectorArray (CallFunction|ReSettingZofArray (select (.Is%20Turn%20Right? (CallFunction|GetSplinePointMidDirectionRight (Variables|Default|GetSpline) (LocalVariables|GetNextIndexRef))) (Utilities|Array|MakeArray (+ (Utilities|Array|Get(acopy) (LocalVariables|GetRightMidRef) (+ (LocalVariables|GetIndexRef) 1)) (* (Math|Vector|GetRightVector (Spline|GetRotationatSplinePoint (Variables|Default|GetSpline) (LocalVariables|GetIndexRef) "Local")) (LocalVariables|GetThickRef) -1.0)) (Utilities|Array|Get(acopy) (LocalVariables|GetRightMidRef) (+ (LocalVariables|GetIndexRef) 1)) (+ (Utilities|Array|Get(acopy) (LocalVariables|GetRightMidRef) (LocalVariables|GetNextIndexRef)) (* (Math|Vector|GetRightVector (Spline|GetRotationatSplinePoint (Variables|Default|GetSpline) (LocalVariables|GetNextIndexRef) "Local")) (LocalVariables|GetThickRef) -1.0)) (Utilities|Array|Get(acopy) (LocalVariables|GetLeftMidRef) (+ (LocalVariables|GetIndexRef) 1))) (Utilities|Array|MakeArray (Utilities|Array|Get(acopy) (LocalVariables|GetLeftMidRef) (+ (LocalVariables|GetIndexRef) 1)) (+ (Utilities|Array|Get(acopy) (LocalVariables|GetLeftMidRef) (+ (LocalVariables|GetIndexRef) 1)) (* (Math|Vector|GetRightVector (Spline|GetRotationatSplinePoint (Variables|Default|GetSpline) (LocalVariables|GetIndexRef) "Local")) (LocalVariables|GetThickRef))) (Utilities|Array|Get(acopy) (LocalVariables|GetRightMidRef) (+ (LocalVariables|GetIndexRef) 1)) (+ (Utilities|Array|Get(acopy) (LocalVariables|GetLeftMidRef) (LocalVariables|GetNextIndexRef)) (* (Math|Vector|GetRightVector (Spline|GetRotationatSplinePoint (Variables|Default|GetSpline) (LocalVariables|GetNextIndexRef) "Local")) (LocalVariables|GetThickRef))))) (.Z (Math|Vector|BreakVector (select (== (LocalVariables|GetIndexRef) (- (Spline|GetNumberOfSplinePoints (Variables|Default|GetSpline)) 2)) (+ (* (Math|Vector|GetRightVector (.rotation _returnvalue_5)) (LocalVariables|GetThickRef) 0.5) (.location _returnvalue_5)) (select (.Is%20Turn%20Right? (CallFunction|GetSplinePointMidDirectionRight (Variables|Default|GetSpline) (+ (LocalVariables|GetIndexRef) 1))) (Utilities|Array|Get(acopy) (LocalVariables|GetRightMidRef) (+ (LocalVariables|GetIndexRef) 1)) (+ (Utilities|Array|Get(acopy) (LocalVariables|GetLeftMidRef) (+ (LocalVariables|GetIndexRef) 1)) (* (Math|Vector|GetRightVector (Spline|GetRotationatSplinePoint (Variables|Default|GetSpline) (LocalVariables|GetIndexRef) "Local")) (LocalVariables|GetThickRef))))))))))))
  (for (_array_element _array_index) (LocalVariables|GetAllWallPoint)
    (bind _returnvalue_6 (DynamicMeshActor|AllocateComputeMesh))
    (bind _returnvalue_7 (Class|GeometryScriptLibraryMeshPrimitiveFunctions|AppendTriangulatedPolygon3D :TargetMesh _returnvalue_6 :PolygonVertices3D (Utilities|Struct|BreakST_VectorArray _array_element) :Debug 0))
    (bind _returnvalue_8 (Class|GeometryScriptLibraryMeshModelingFunctions|ApplyMeshLinearExtrudeFaces :TargetMesh _returnvalue_7 :Options (Utilities|Struct|MakeGeometryScriptMeshLinearExtrudeOptions (.z (LocalVariables|GetHandleLoc)) "FixedDirection") :Debug 0))
    (bind _returnvalue_9 (DynamicMeshActor|AllocateComputeMesh))
    (bind _returnvalue_10 (Class|GeometryScriptLibraryMeshPrimitiveFunctions|AppendTriangulatedPolygon3D :TargetMesh _returnvalue_9 :PolygonVertices3D (Utilities|Struct|BreakST_VectorArray (Utilities|Array|Get(acopy) (LocalVariables|GetAll%20corner%20Point) _array_index)) :Debug 0))
    (bind _returnvalue_11 (Class|GeometryScriptLibraryMeshModelingFunctions|ApplyMeshLinearExtrudeFaces :TargetMesh _returnvalue_10 :Options (Utilities|Struct|MakeGeometryScriptMeshLinearExtrudeOptions (.z (LocalVariables|GetHandleLoc)) "FixedDirection") :Debug 0))
    (Class|GeometryScriptLibraryMeshNormalsFunctions|FlipNormals _returnvalue_11 0)
    (bind _returnvalue_12 (GeometryScript|MeshEdits|AppendMesh :TargetMesh _returnvalue_11 :AppendMesh _returnvalue_8 :AppendOptions "(CombineMode=EnableAllMatching)" :Debug 0))
    (bind _returnvalue_13 (Class|GeometryScriptLibraryMeshUVFunctions|SetMeshUVsfromBoxProjection :TargetMesh _returnvalue_12 :BoxTransform (Math|Transform|MakeTransform (select _mat_world_align_ (Math|Transform|InverseTransformLocation _returnvalue "0, 0, 0") (.location (Spline|GetTransformatSplinePoint (Variables|Default|GetSpline) _array_index "Local" false))) (select _mat_world_align_ (Math|Transform|InverseTransformRotation _returnvalue "0, 0, 0") (.rotation (Spline|GetTransformatSplinePoint (Variables|Default|GetSpline) _array_index "Local" false))) "100.000000,100.000000,100.000000") :Debug 0))
    (GeometryScript|MeshEdits|AppendMesh :TargetMesh (Variables|Default|GetDynmesh) :AppendMesh _returnvalue_13 :AppendOptions "(CombineMode=EnableAllMatching)" :Debug 0)))

(fn GetSplinePointHorizontalAngle
  (params (index :type Integer) (spline :type Spline%20Component%20Object%20Reference))
  (bind _returnvalue (Spline|GetLocationatSplinePoint spline index "Local"))
  (return (Class|KismetMathLibrary|DegAcos (Math|Vector2D|DotProduct(2D) (Math|Conversions|ToVector2D(Vector) (Math|Vector|GetUnitDirection(Vector) _returnvalue (Spline|GetLocationatSplinePoint spline (+ index -1) "Local"))) (Math|Conversions|ToVector2D(Vector) (Math|Vector|GetUnitDirection(Vector) _returnvalue (Spline|GetLocationatSplinePoint spline (+ index 1) "Local")))))))

(fn ReSettingZofArray
  (params (Array :type Array%20of%20Vectors) (Z :type Float%20%28double-precision%29))
  (bind _arrayelement (Utilities|Array|ReverseforEachLoop Array)
    (:LoopBody
      (Utilities|Array|Add (LocalVariables|GetREE) (Math|Vector|MakeVector (.X (Math|Vector|BreakVector _arrayelement)) (.Y (Math|Vector|BreakVector _arrayelement)) Z)))
    (:Completed
      (return (LocalVariables|GetREE)))))

(fn SnapCheck
  (bind _spline (Variables|Default|GetSpline))
  (bind _handle (Variables|Default|GetHandle))
  (bind _returnvalue (* (.z (.location _handle)) 0.51))
  (for _index (range 0 (- (Spline|GetNumberOfSplinePoints (Variables|Default|GetSpline)) 2))
    (bind (_outhits _returnvalue_2) (Class|KismetSystemLibrary|BoxTraceMultiforObjects (+ (CallFunction|ReturntoCenterPoint (Spline|GetLocationatSplinePoint _spline _index "World") (Spline|GetLocationatSplinePoint _spline (+ _index 1) "World")) (Math|Vector|MakeVector 0.0 0.0 _returnvalue)) (+ (CallFunction|ReturntoCenterPoint (Spline|GetLocationatSplinePoint _spline _index "World") (Spline|GetLocationatSplinePoint _spline (+ _index 1) "World")) (Math|Vector|MakeVector 0.0 0.0 _returnvalue)) (Math|Vector|MakeVector (Math|Vector|Distance(Vector) (Spline|GetLocationatSplinePoint _spline _index "World") (CallFunction|ReturntoCenterPoint (Spline|GetLocationatSplinePoint _spline _index "World") (Spline|GetLocationatSplinePoint _spline (+ _index 1) "World"))) (+ (Math|Vector|Distance2D(Vector) (.location (Variables|Default|GetHandle)) "0, 0, 0") 2.0) _returnvalue) (Spline|GetRotationatSplinePoint (Variables|Default|GetSpline) _index "World") (Utilities|Array|MakeArray "ObjectTypeQuery2" "ObjectTypeQuery1") true 0 "ForOneFrame" true))
    (if _returnvalue_2
      (bind _returnvalue_3 (DynamicMeshActor|AllocateComputeMesh))
      (LocalVariables|SettoolR _returnvalue_3)
      (for _array_element _outhits
        (Development|PrintString (Utilities|GetDisplayName (.HitActor (Collision|BreakHitResult _array_element))) true false)
        (bind _dynmesh (Class|BPISnapBoole|GetBooleMeshData(Message) (.HitActor (Collision|BreakHitResult _array_element))))
        (if (and (.HasBooleRequire? (Utilities|Struct|BreakST_BooleSnapData _dynmesh)) (Utilities|Array|ContainsItem (.SnapedActor (Utilities|Struct|BreakST_BooleSnapData _dynmesh)) self))
          (GeometryScript|MeshEdits|AppendMesh (LocalVariables|GettoolR) (.DynMash (Utilities|Struct|BreakST_BooleSnapData _dynmesh)) (.Tar (Utilities|Struct|BreakST_BooleSnapData _dynmesh)) false "(CombineMode=EnableAllMatching)" 0)))
      (GeometryScript|Booleans|ApplyMeshBoolean :TargetMesh (Variables|Default|GetDynmesh) :ToolMesh (LocalVariables|GettoolR) :Operation "Subtract" :Options (Utilities|Struct|MakeGeometryScriptMeshBooleanOptions false true 0.01 false) :Debug 0))))

(fn ReturntoCenterPoint
  (params (A :type Vector) (B :type Vector))
  (return (+ A (* (Math|Rotator|GetRotationXVector (Math|Rotator|FindLookatRotation A B)) (* (Math|Vector|Distance(Vector) A B) 0.5)))))

(fn GetBooleMeshData
  (return ""))

(fn GetCanbeSnapBoolePlaneData
  (return 0 (* (Math|Vector|Distance2D(Vector) (.location (Variables|Default|GetHandle)) "0, 0, 0") 2.0)))