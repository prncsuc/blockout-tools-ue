(event Custom|Build
  (bind _materialconfigurationarray (Variables|Default|GetMaterialConfigurationArray))
  (bind _dynamicmeshcomponent (Variables|DynamicMeshActor|GetDynamicMeshComponent))
  (Components|DestroyComponent (Actor|GetComponentsByClass "/Script/Engine.ChildActorComponent"))
  (DynamicMeshActor|ReleaseAllComputeMeshes)
  ;[0 0 0] Reset material
  (Utilities|Array|Clear (Variables|Default|GetMaterialConfigurationArray))
  (for _index (range 0 (- (Rendering|Material|GetNumMaterials _dynamicmeshcomponent) 1))
    (Rendering|Material|SetMaterial _dynamicmeshcomponent _index 0))
  (Class|DynamicMeshComponent|ValidateMaterialSlots _dynamicmeshcomponent true true)
  (bind _returnvalue (DynamicMeshActor|AllocateComputeMesh))
  (bind _output_get (Variables|Default|SetDynmesh _returnvalue))
  (bind _returnvalue_2 (Class|GeometryScriptLibraryMeshPrimitiveFunctions|AppendTriangulatedPolygon3D :TargetMesh _output_get :PolygonVertices3D (Utilities|Array|MakeArray "0, 0, 0" (Math|Vector|MakeVector 0.0 0.0 (.z (Variables|Default|GetHandleUp))) (Math|Vector|MakeVector (.x (Variables|Default|GetHandleF)) 0.0 0.0)) :Debug 0))
  (bind _returnvalue_3 (Class|GeometryScriptLibraryMeshModelingFunctions|ApplyMeshLinearExtrudeFaces :TargetMesh _returnvalue_2 :Options (Utilities|Struct|MakeGeometryScriptMeshLinearExtrudeOptions (.y (Variables|Default|GetHandleF)) "FixedDirection" "0.000000,1.000000,0.000000" "EntireSelection" "(GroupMode=PreserveExisting,ConstantGroup=0)" 1.0 true) :Debug 0))
  (Class|GeometryScriptLibraryMeshNormalsFunctions|FlipNormals _returnvalue_3 0)
  (bind _returnvalue_4 (Class|GeometryScriptLibraryMeshNormalsFunctions|ComputeSplitNormals :TargetMesh _returnvalue_3 :SplitOptions (Utilities|Struct|MakeGeometryScriptSplitNormalsOptions true 15.0 false "(bDefaultLayer=True,ExtendedLayerIndex=0)") :Debug 0))
  (Utilities|FlowControl|Sequence
    (:then_0
      (if (Variables|Default|Getmirror)
        (bind _returnvalue_5 (DynamicMeshActor|AllocateComputeMesh))
        (bind _returnvalue_6 (Class|GeometryScriptLibraryMeshDecompositionFunctions|CopyMeshSelectiontoMesh :TargetMesh _returnvalue_4 :StoreToSubmesh _returnvalue_5 :Debug 0))
        (GeometryScript|MeshEdits|AppendMesh (Variables|Default|GetDynmesh) _returnvalue_6 (Math|Transform|MakeTransform (Math|Vector|MakeVector 0.0 (.y (Variables|Default|GetHandleF)) 0.0) "0.000000,180.000000,0.000000" "1.000000,1.000000,1.000000") false "(CombineMode=EnableAllMatching)" 0)))
    (:then_1
      (Utilities|Array|Add (Variables|Default|GetMaterialConfigurationArray) (CallFunction|CreateandSetDynamicMaterials (Variables|Default|GetMateral) (Variables|Default|GetColor%20Set) "None"))
      (Class|DynamicMeshComponent|SetDynamicMesh (Variables|DynamicMeshActor|GetDynamicMeshComponent) (Variables|Default|GetDynmesh))
      ;[0 0 0] When the material of the component is not set, it is set to the primary material
      (for (_array_element _array_index) _materialconfigurationarray
        (if (not (Utilities|IsValid _array_element))
          (Utilities|Array|SetArrayElem _materialconfigurationarray _array_index (CallFunction|CreateandSetDynamicMaterials (Variables|Default|GetMateral) (Variables|Default|GetColor%20Set) "None"))))
      (Class|DynamicMeshComponent|ConfigureMaterialSet (Variables|DynamicMeshActor|GetDynamicMeshComponent) (Variables|Default|GetMaterialConfigurationArray)))))

(fn ConstructionScript
  (Variables|Default|SetHandleUp (Math|Vector|MakeVector 0.0 0.0 (select (< (.z (Variables|Default|GetHandleUp)) 0.0) 0.0 (.z (Variables|Default|GetHandleUp)))))
  (Variables|Default|SetHandleF (Math|Vector|MakeVector (.x (Variables|Default|GetHandleF)) (.y (Variables|Default|GetHandleF)) 0.0))
  (Utilities|FlowControl|Sequence
    (:then_0
      (if (Variables|Default|GetArrowSnap?)
        (Utilities|FlowControl|Sequence
          (:then_0
            (Transformation|SetRelativeLocation (Variables|Default|GetZ-SnapArrow) (CallFunction|ReturntoCenterPoint (Variables|Default|GetHandleF) "0, 0, 0") false false)
            (Transformation|SetRelativeLocation (Variables|Default|GetX-SnapArrow) (CallFunction|ReturntoCenterPoint (Math|Vector|MakeVector 0.0 (.y (Variables|Default|GetHandleF)) (.z (Variables|Default|GetHandleUp))) "0, 0, 0") false false)
            (Transformation|SetRelativeLocation (Variables|Default|GetY-SnapArrow1) (Math|Vector|GetVectorArrayAverage (Utilities|Array|MakeArray (Variables|Default|GetHandleUp) "0, 0, 0" (Math|Vector|MakeVector (.x (Variables|Default|GetHandleF)) 0.0 0.0))) false false)
            (Transformation|SetRelativeLocation (Variables|Default|GetY+SnapArrow1) (Math|Vector|GetVectorArrayAverage (Utilities|Array|MakeArray (Math|Vector|MakeVector (.x (Variables|Default|GetHandleUp)) (.y (Variables|Default|GetHandleF)) (.z (Variables|Default|GetHandleUp))) (Math|Vector|MakeVector 0.0 (.y (Variables|Default|GetHandleF)) 0.0) (Math|Vector|MakeVector (.x (Variables|Default|GetHandleF)) (.y (Variables|Default|GetHandleF)) 0.0))) false false))
          (:then_1
            (bind _offset (CallFunction|ArrowsSnapCheck (Variables|Default|GetCheckArrows)))
            (for _array_element _offset
              (Transformation|AddActorWorldOffset _array_element))))
        (else
          (for _array_element_2 (Components|GetChildrenComponents (Variables|Default|GetCheckArrows) true)
            (Rendering|SetVisibility _array_element_2 false false)))))
    (:then_2
      (if (Variables|Default|GetVertex%20Snap?)
        (Utilities|FlowControl|Sequence
          (:then_0
            (bind (_scd _reloc _rew) (CallFunction|DynActorVertexSnapCheck "0, 0, 0" 1e+01))
            (if _scd
              (Transformation|SetActorLocation _rew false false)))
          (:then_1
            (bind (_scd_2 _reloc_2) (CallFunction|DynActorVertexSnapCheck (Variables|Default|GetHandleUp) 1e+01))
            (if _scd_2
              (Variables|Default|SetHandleUp _reloc_2)))
          (:then_2
            (bind (_scd_3 _reloc_3) (CallFunction|DynActorVertexSnapCheck (Math|Vector|MakeVector 0.0 (.y (Variables|Default|GetHandleF)) 0.0) 1e+01))
            (if _scd_3
              (Variables|Default|SetHandleF (Math|Vector|MakeVector (.x (Variables|Default|GetHandleF)) (.Y (Math|Vector|BreakVector _reloc_3)) 0.0)))))))
    (:then_3
      (CallFunction|Build))))

(fn CreateandSetDynamicMaterials
  (params (Materal :type Material%20Interface%20Object%20Reference) (ColorSet :type ST%20Color%20Set%20V2%20Structure) (OptionalName :type Name))
  (bind (_enableset _texture _normaltex _hue _saturation _light _rough _coloroverlay _tlie _rotate) (Utilities|Struct|BreakST_ColorSetV2 ColorSet))
  (bind _returnvalue (Rendering|Material|CreateDynamicMaterialInstance (Variables|DynamicMeshActor|GetDynamicMeshComponent) (Utilities|Array|Length (Variables|Default|GetMaterialConfigurationArray)) (select (Utilities|IsValid Materal) Materal "/Game/PMB/BlockoutToolKit/Materials/Adjustable/MI_PMB_Adj__cement.MI_PMB_Adj__cement") OptionalName :!class /Script/Engine.PrimitiveComponent))
  (if _enableset
    (Rendering|Material|SetVectorParameterValue _returnvalue "Color" (Utilities|Struct|MakeLinearColor _hue _saturation _light _rough) :!class /Script/Engine.MaterialInstanceDynamic)
    (Rendering|Material|SetTextureParameterValue _returnvalue "Texture" _texture)
    (Rendering|Material|SetTextureParameterValue _returnvalue "Normal" _normaltex)
    (Rendering|Material|SetScalarParameterValue _returnvalue "Tlie" (Math|Conversions|ToFloat(Integer) _tlie) :!class /Script/Engine.MaterialInstanceDynamic)
    (Rendering|Material|SetScalarParameterValue _returnvalue "rotate" (Math|Float|MapRangeClamped (Math|Conversions|ToFloat(Integer) _rotate) 0.0 3.6e+02 0.0 1.0) :!class /Script/Engine.MaterialInstanceDynamic)
    (Rendering|Material|SetVectorParameterValue _returnvalue "ColorOverlay" _coloroverlay :!class /Script/Engine.MaterialInstanceDynamic))
  (return _returnvalue))

(fn DynActorVertexSnapCheck
  (params (LocIn :type Vector) (Check%20Radius :type Float%20%28double-precision%29))
  (bind _returnvalue (Transformation|GetActorTransform))
  (bind _returnvalue_2 (Math|Transform|TransformLocation _returnvalue LocIn))
  (LocalVariables|SetPointW _returnvalue_2)
  (bind _outhits (Collision|MultiSphereTraceForObjects _returnvalue_2 _returnvalue_2 Check%20Radius (Utilities|Array|MakeArray "ObjectTypeQuery1" "ObjectTypeQuery2") false 0 "ForOneFrame"))
  (for _array_element _outhits
    (bind _asdynamic_mesh_actor (Utilities|Casting|CastToDynamicMeshActor (.HitActor (Collision|BreakHitResult _array_element))))
    (bind _returnvalue_3 (DynamicMeshComponent|GetDynamicMesh (Variables|/Script/GeometryFramework.DynamicMeshActor|GetDynamicMeshComponent _asdynamic_mesh_actor)))
    (bind _positionlist (GeometryScript|MeshQueries|GetAllVertexPositions _returnvalue_3))
    (bind _vectorarray (Class|GeometryScriptLibraryListUtilityFunctions|ConvertVectorListtoArray _positionlist))
    (for _array_element_2 _vectorarray
      (if (< (Math|Vector|Distance(Vector) (LocalVariables|GetPointW) (Math|Transform|TransformLocation (Transformation|GetActorTransform (.HitActor (Collision|BreakHitResult _array_element))) _array_element_2)) Check%20Radius)
        (return true (Math|Transform|InverseTransformLocation (Transformation|GetActorTransform) (Math|Transform|TransformLocation (Transformation|GetActorTransform (.HitActor (Collision|BreakHitResult _array_element))) _array_element_2)) (Math|Transform|TransformLocation (Transformation|GetActorTransform (.HitActor (Collision|BreakHitResult _array_element))) _array_element_2)))))
  (return false "0, 0, 0" "0, 0, 0"))

(fn ArrowsSnapCheck
  (params (Arrows%20RootCom :type Scene%20Component%20Object%20Reference))
  (bind _arrayelement (Utilities|Array|ReverseforEachLoop (Components|GetChildrenComponents Arrows%20RootCom true))
    (:LoopBody
      (bind _asarrow_component (Utilities|Casting|CastToArrowComponent _arrayelement))
      (bind (_outhit _returnvalue) (Collision|LineTraceByChannel (Transformation|GetWorldLocation _asarrow_component) (+ (Transformation|GetWorldLocation _asarrow_component) (* (Math|Vector|GetForwardVector _asarrow_component) (Variables|/Script/Engine.ArrowComponent|GetArrowLength _asarrow_component))) "TraceTypeQuery1" true 0 "ForOneFrame"))
      (Utilities|Array|Add (LocalVariables|GetOffsetArray) (select _returnvalue (- (.Location (Collision|BreakHitResult _outhit)) (.TraceStart (Collision|BreakHitResult _outhit))) "0, 0, 0")))
    (:Completed
      (return (LocalVariables|GetOffsetArray)))))

(fn ReturntoCenterPoint
  (params (A :type Vector) (B :type Vector))
  (return (+ A (* (Math|Rotator|GetRotationXVector (Math|Rotator|FindLookatRotation A B)) (* (Math|Vector|Distance(Vector) A B) 0.5)))))