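; Base Blueprint for blockout props that snap to surfaces and can supply a boolean cutter to the host actor.
; Its construction script flattens the linear spline to a local plane, line-traces along child arrows, snaps to BPI_SnapBoole actors along the hit normal, and notifies current and previous hosts to update.
; GetBooleMeshData uses Geometry Script to extrude the spline polygon into a cutter mesh, returned with a host-relative transform.
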(fn ConstructionScript
  (bind _boolespline (Variables|Default|GetBooleSpline))
  (for _index (range 0 (- (Spline|GetNumberOfSplinePoints _boolespline) 1))
    (Spline|SetSplinePointType _boolespline _index "Linear" false)
    (Spline|SetLocationatSplinePoint _boolespline _index (Math|Vector|MakeVector 0.0 (.Y (Math|Vector|BreakVector (Spline|GetLocationatSplinePoint _boolespline _index "Local"))) (.Z (Math|Vector|BreakVector (Spline|GetLocationatSplinePoint _boolespline _index "Local")))) "Local" true))
  (bind (_outhit _scd _arrayelement) (CallFunction|SnapCheck))
  (if _scd
    (if (Utilities|DoesObjectImplementInterface (.HitActor (Collision|BreakHitResult _outhit)) "/Game/PMB/BlockoutToolKit/Interface/BPI_SnapBoole.BPI_SnapBoole_C")
      (bind _boole_to_actor (Variables|Default|GetBoole%20To%20Actor)
        (:then
          (Class|BPISnapBoole|SendUpdatedBooleanEventOfSnapPerson(Message) _boole_to_actor))
        (:else
          _))
      (Variables|Default|SetBoole%20To%20Actor (.HitActor (Collision|BreakHitResult _outhit)))
      (Transformation|SetActorTransform (Math|Transform|MakeTransform (+ (.Location (Collision|BreakHitResult _outhit)) (* (Math|Vector|GetForwardVector (Math|Rotator|MakeRotfromX (.Normal (Collision|BreakHitResult _outhit)))) (.x (.location (Transformation|GetRelativeTransform _arrayelement))) -1.0) (* (Math|Vector|GetRightVector (Math|Rotator|MakeRotfromX (.Normal (Collision|BreakHitResult _outhit)))) (.y (.location (Transformation|GetRelativeTransform _arrayelement))) -1.0) (* (Math|Vector|GetUpVector (Math|Rotator|MakeRotfromX (.Normal (Collision|BreakHitResult _outhit)))) (.z (.location (Transformation|GetRelativeTransform _arrayelement))) -1.0)) (Math|Rotator|MakeRotfromX (.Normal (Collision|BreakHitResult _outhit))) "1.000000,1.000000,1.000000"))
      (if (Variables|Default|GetBoole?)
        (Class|BPISnapBoole|SendUpdatedBooleanEventOfSnapPerson(Message) (.HitActor (Collision|BreakHitResult _outhit)))))
    (else
      (bind _boole_to_actor_2 (Variables|Default|GetBoole%20To%20Actor)
        (:then
          (Class|BPISnapBoole|SendUpdatedBooleanEventOfSnapPerson(Message) _boole_to_actor_2))
        (:else)))))

(fn SnapCheck
  (bind _arrayelement (Utilities|Array|ReverseforEachLoop (Components|GetChildrenComponents (Variables|Default|GetCheckArray) false))
    (:LoopBody
      (bind _asarrow_component (Utilities|Casting|CastToArrowComponent _arrayelement))
      (bind (_outhit _returnvalue) (Collision|LineTraceForObjects (+ (Transformation|GetWorldLocation _asarrow_component) (* (* (Math|Vector|GetForwardVector _asarrow_component) (Variables|/Script/Engine.ArrowComponent|GetArrowLength _asarrow_component)) -1.0)) (+ (Transformation|GetWorldLocation _asarrow_component) (* (Math|Vector|GetForwardVector _asarrow_component) (Variables|/Script/Engine.ArrowComponent|GetArrowLength _asarrow_component))) (Utilities|Array|MakeArray "ObjectTypeQuery1") true 0 "ForOneFrame"))
      (if _returnvalue
        (return _outhit true _arrayelement)))
    (:Completed
      (return "" false 0))))

(fn GetBooleMeshData
  (bind _boole_to_actor (Variables|Default|GetBoole%20To%20Actor))
  (bind _boolespline (Variables|Default|GetBooleSpline))
  (bind _returnvalue (Transformation|GetActorTransform _boole_to_actor))
  (for _index (range 0 (- (Spline|GetNumberOfSplinePoints _boolespline) 1))
    (Utilities|Array|Add (LocalVariables|GetArray) (+ (Spline|GetLocationatSplinePoint _boolespline _index "World") (* (Math|Vector|GetForwardVector (Transformation|GetActorRotation)) (Variables|Default|GetBoole%20Thick)))))
  (bind _returnvalue_2 (DynamicMeshActor|AllocateComputeMesh))
  (bind _returnvalue_3 (Class|GeometryScriptLibraryMeshPrimitiveFunctions|AppendTriangulatedPolygon3D :TargetMesh _returnvalue_2 :PolygonVertices3D (LocalVariables|GetArray) :Debug 0))
  (bind _returnvalue_4 (Class|GeometryScriptLibraryMeshModelingFunctions|ApplyMeshLinearExtrudeFaces :TargetMesh _returnvalue_3 :Options (Utilities|Struct|MakeGeometryScriptMeshLinearExtrudeOptions (* (Variables|Default|GetBoole%20Thick) 2.0) "FixedDirection" (* (Math|Vector|GetForwardVector (Transformation|GetActorRotation)) -2.0)) :Debug 0))
  (return (Utilities|Struct|MakeST_BooleSnapData (Variables|Default|GetBoole?) (Math|Transform|MakeTransform (Math|Transform|InverseTransformLocation _returnvalue "0, 0, 0") (Math|Transform|InverseTransformRotation _returnvalue "0, 0, 0")) _returnvalue_4 (Utilities|Array|MakeArray (Variables|Default|GetBoole%20To%20Actor)))))

(fn GetCanbeSnapBoolePlaneData
  (return 0 0.0))