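; Blockout toolkit snap-prop door that swings open and shut as the player enters its trigger volumes.
; Two open triggers set a Flip flag so the door mesh rotates 90 degrees in either direction, and two close triggers return it to zero rotation.
; Timelines drive both rotation lerps, while running and open-state flags block overlapping or repeated moves.
; Construction defers to the parent class.
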(event OnComponentBeginOverlap(Open)
  (params (OverlappedComponent :type Primitive%20Component%20Object%20Reference) (OtherActor :type Actor%20Object%20Reference) (OtherComp :type Primitive%20Component%20Object%20Reference) (OtherBodyIndex :type Integer) (bFromSweep :type Boolean) (SweepResult :type Hit%20Result%20Structure%20%28by%20ref%29))
  (if (== OtherActor (Game|GetPlayerCharacter 0))
    (if (not (Variables|Default|GetRuning？))
      (if (not (Variables|Default|GetIs%20Open？))
        (Variables|Default|SetFlip? false)
        (CallFunction|OpenDoor)))))

(event OnComponentBeginOverlap(Close1)
  (params (OverlappedComponent :type Primitive%20Component%20Object%20Reference) (OtherActor :type Actor%20Object%20Reference) (OtherComp :type Primitive%20Component%20Object%20Reference) (OtherBodyIndex :type Integer) (bFromSweep :type Boolean) (SweepResult :type Hit%20Result%20Structure%20%28by%20ref%29))
  (if (== OtherActor (Game|GetPlayerCharacter 0))
    (if (not (Variables|Default|GetRuning？))
      (if (Variables|Default|GetIs%20Open？)
        (CallFunction|CloseDoor)))))

(event OnComponentBeginOverlap(Poen1)
  (params (OverlappedComponent :type Primitive%20Component%20Object%20Reference) (OtherActor :type Actor%20Object%20Reference) (OtherComp :type Primitive%20Component%20Object%20Reference) (OtherBodyIndex :type Integer) (bFromSweep :type Boolean) (SweepResult :type Hit%20Result%20Structure%20%28by%20ref%29))
  (if (== OtherActor (Game|GetPlayerCharacter 0))
    (if (not (Variables|Default|GetRuning？))
      (if (not (Variables|Default|GetIs%20Open？))
        (Variables|Default|SetFlip? true)
        (CallFunction|OpenDoor)))))

(event OnComponentBeginOverlap(Close)
  (params (OverlappedComponent :type Primitive%20Component%20Object%20Reference) (OtherActor :type Actor%20Object%20Reference) (OtherComp :type Primitive%20Component%20Object%20Reference) (OtherBodyIndex :type Integer) (bFromSweep :type Boolean) (SweepResult :type Hit%20Result%20Structure%20%28by%20ref%29))
  (if (== OtherActor (Game|GetPlayerCharacter 0))
    (if (not (Variables|Default|GetRuning？))
      (if (Variables|Default|GetIs%20Open？)
        (CallFunction|CloseDoor)))))

(event Custom|CloseDoor
  (if (not (Variables|Default|GetRuning？))
    (Variables|Default|SetRuning？ true)
    (Variables|Default|SetRotote (.rotation (Transformation|GetRelativeTransform (Variables|Default|GetSM_Door))))
    (bind _1 (Timeline|时间轴 PlayFromStart)
      (:Update
        (Transformation|SetRelativeRotation (Variables|Default|GetSM_Door) (Math|Rotator|Lerp(Rotator) (Variables|Default|GetRotote) "0, 0, 0" _1 true) false false))
      (:Finished
        (Variables|Default|SetIs%20Open？ false)
        (Variables|Default|SetRuning？ false)))))

(event Custom|OpenDoor
  (if (not (Variables|Default|GetRuning？))
    (Variables|Default|SetRuning？ true)
    (bind _1 (Timeline|OpenDoor1 PlayFromStart)
      (:Update
        (Transformation|SetRelativeRotation (Variables|Default|GetSM_Door) (select (Variables|Default|GetFlip?) (Math|Rotator|Lerp(Rotator) "0, 0, 0" "0.000000,90.000000,0.000000" _1 true) (Math|Rotator|Lerp(Rotator) "0, 0, 0" "0.000000,-90.000000,0.000000" _1 true)) false false))
      (:Finished
        (Variables|Default|SetIs%20Open？ true)
        (Variables|Default|SetRuning？ false)))))

(fn ConstructionScript
  (|CallParentFunction))