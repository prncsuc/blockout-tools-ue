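; Level-design blockout actor that turns a spline outline into an extruded polygon prism in the editor.
; On construction, unless booled, it flattens linear spline points, triangulates and extrudes them to the Handle height, and insets one cap by a retract amount for tapering.
; It applies dynamic materials with optional colour and texture overrides.
; It can supply its untapered mesh as boolean data, but its trace-based surface-snapping logic is unconnected.
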(event Custom|Build
  (bind _materialconfigurationarray (Variables|Default|GetMaterialConfigurationArray))
  (bind _dynamicmeshcomponent (Variables|DynamicMeshActor|GetDynamicMeshComponent))
  (Variables|Default|Sethandle (Math|Vector|MakeVector 0.0 0.0 (.z (Variables|Default|Gethandle))))
  (DynamicMeshActor|ReleaseAllComputeMeshes)
  (if (not (Variables|Default|GetIs%20Booled))
    ;[0 0 0] Reset material
    (Utilities|Array|Clear (Variables|Default|GetMaterialConfigurationArray))
    (for _index (range 0 (- (Rendering|Material|GetNumMaterials _dynamicmeshcomponent) 1))
      (Rendering|Material|SetMaterial _dynamicmeshcomponent _index 0))
    (Class|DynamicMeshComponent|ValidateMaterialSlots _dynamicmeshcomponent true true)
    (bind _pointarray (CallFunction|SplinePreWork))
    (bind _returnvalue (DynamicMeshActor|AllocateComputeMesh))
    (bind _returnvalue_2 (Class|GeometryScriptLibraryMeshPrimitiveFunctions|AppendTriangulatedPolygon3D :TargetMesh _returnvalue :PolygonVertices3D _pointarray :Debug 0))
    (bind _returnvalue_3 (Class|GeometryScriptLibraryMeshModelingFunctions|ApplyMeshLinearExtrudeFaces :TargetMesh _returnvalue_2 :Options (Utilities|Struct|MakeGeometryScriptMeshLinearExtrudeOptions (.z (Variables|Default|Gethandle)) "FixedDirection" "0.000000,0.000000,1.000000" "EntireSelection" "(GroupMode=PreserveExisting,ConstantGroup=0)" 1.0 true) :Debug 0))
    (Utilities|Array|Add (Variables|Default|GetMaterialConfigurationArray) (CallFunction|CreateandSetDynamicMaterials (Variables|Default|GetMateral) (Variables|Default|GetColor%20Set) "None"))
    (for (_array_element _array_index) (.Re (CallFunction|GetSplinePointArray (Variables|Default|GetSpline) "Local" (Variables|Default|GetRectract) 0.0 true))
      (Class|GeometryScriptLibraryMeshBasicEditFunctions|SetVertexPosition _returnvalue_3 _array_index (Math|Vector|MakeVector (.X (Math|Vector|BreakVector _array_element)) (.Y (Math|Vector|BreakVector _array_element)) (.z (Variables|Default|Gethandle))) false))
    (Utilities|FlowControl|Sequence
      (:then_0
        (if (!= (Variables|Default|GetRectract) 0.0)
          (Class|GeometryScriptLibraryMeshUVFunctions|SetMeshUVsfromPlanarProjection :TargetMesh _returnvalue_3 :PlaneTransform (Math|Transform|MakeTransform "0, 0, 0" "0, 0, 0" "100.000000,100.000000,100.000000") :Debug 0)))
      (:then_1
        (Class|DynamicMeshComponent|SetDynamicMesh (Variables|DynamicMeshActor|GetDynamicMeshComponent) _returnvalue_3)
        ;[0 0 0] When the material of the component is not set, it is set to the primary material
        (for (_array_element_2 _array_index_2) _materialconfigurationarray
          (if (not (Utilities|IsValid _array_element_2))
            (Utilities|Array|SetArrayElem _materialconfigurationarray _array_index_2 (CallFunction|CreateandSetDynamicMaterials (Variables|Default|GetMateral) (Variables|Default|GetColor%20Set) "None"))))
        (Class|DynamicMeshComponent|ConfigureMaterialSet (Variables|DynamicMeshActor|GetDynamicMeshComponent) (Variables|Default|GetMaterialConfigurationArray))))))

(fn ConstructionScript
  (CallFunction|Build))

(fn SnapCheck
  (bind _arrayelement (Utilities|Array|ReverseforEachLoop (Components|GetChildrenComponents (Variables|Default|GetCheckArray) false))
    (:LoopBody
      (bind _asarrow_component (Utilities|Casting|CastToArrowComponent _arrayelement))
      (bind (_outhit _returnvalue) (Collision|LineTraceForObjects (+ (Transformation|GetWorldLocation _asarrow_component) (* (* (Math|Vector|GetForwardVector _asarrow_component) (Variables|/Script/Engine.ArrowComponent|GetArrowLength _asarrow_component)) -1.0)) (+ (Transformation|GetWorldLocation _asarrow_component) (* (Math|Vector|GetForwardVector _asarrow_component) (Variables|/Script/Engine.ArrowComponent|GetArrowLength _asarrow_component))) (Utilities|Array|MakeArray "ObjectTypeQuery1") true 0 "ForOneFrame"))
      (if _returnvalue
        (return _outhit true _arrayelement)))
    (:Completed
      (return "" false 0))))

(fn SplinePreWork
  (bind _spline (Variables|Default|GetSpline))
  (for _index (range 0 (- (Spline|GetNumberOfSplinePoints _spline) 1))
    (Spline|SetSplinePointType _spline _index "Linear" false)
    (Spline|SetLocationatSplinePoint _spline _index (Math|Vector|MakeVector (.X (Math|Vector|BreakVector (Spline|GetLocationatSplinePoint _spline _index "Local"))) (.Y (Math|Vector|BreakVector (Spline|GetLocationatSplinePoint _spline _index "Local"))) 0.0) "Local" true)
    (Utilities|Array|Add (LocalVariables|GetArray) (Math|Vector|MakeVector (.X (Math|Vector|BreakVector (Spline|GetLocationatSplinePoint _spline _index "Local"))) (.Y (Math|Vector|BreakVector (Spline|GetLocationatSplinePoint _spline _index "Local"))) 0.0)))
  (return (LocalVariables|GetArray)))

(fn CreateandSetDynamicMaterials
  (params (Materal :type Material%20Interface%20Object%20Reference) (ColorSet :type ST%20Color%20Set%20V2%20Structure) (OptionalName :type Name))
  (bind (_enableset _texture _normaltex _hue _saturation _light _rough _coloroverlay _tlie _rotate) (Utilities|Struct|BreakST_ColorSetV2 ColorSet))
  (bind _returnvalue (Rendering|Material|CreateDynamicMaterialInstance (Variables|DynamicMeshActor|GetDynamicMeshComponent) (Utilities|Array|Length (Variables|Default|GetMaterialConfigurationArray)) (select (Utilities|IsValid Materal) Materal "/Game/PMB/BlockoutToolKit/Materials/Adjustable/MI_PMB_Adj__cement.MI_PMB_Adj__cement") OptionalName :!class /Script/Engine.PrimitiveComponent))
  (if _enableset
    (Rendering|Material|SetVectorParameterValue _returnvalue "Color" (Utilities|Struct|MakeLinearColor _hue _saturation _light _rough) :!class /Script/Engine.MaterialInstanceDynamic)
    (Rendering|Material|SetTextureParameterValue _returnvalue "Texture" _texture)
    (Rendering|Material|SetTextureParameterValue _returnvalue "Normal" _normaltex)
    (Rendering|Material|SetScalarParameterValue _returnvalue "Tlie" (Math|Conversions|ToFloat(Integer) _tlie) :!class /Script/Engine.MaterialInstanceDynamic)
    (Rendering|Material|SetScalarParameterValue _returnvalue "rotate" (Math|Float|MapRangeClamped (Math|Conversions|ToFloat(Integer) _rotate) 0.0 3.6e+02 0.0 1.0) :!class /Script/Engine.MaterialInstanceDynamic)
    (Rendering|Material|SetVectorParameterValue _returnvalue "ColorOverlay" _coloroverlay :!class /Script/Engine.MaterialInstanceDynamic))
  (return _returnvalue))

(fn GetNextSplinePoint
  (params (Current%20index :type Integer) (next？ :type Boolean))
  (bind _returnvalue (+ Current%20index 1))
  (if next？
    (return (select (== _returnvalue (Spline|GetNumberOfSplinePoints (Variables|Default|GetSpline))) 0 _returnvalue))
    (else
      (return (select (== Current%20index 0) (- (Spline|GetNumberOfSplinePoints (Variables|Default|GetSpline)) 1) (- Current%20index 1))))))

(fn GetSplinePointMidDirectionRight
  (params (Spline :type Spline%20Component%20Object%20Reference) (PointIndex :type Integer) (CloseMode? :type Boolean))
  (bind _returnvalue (Spline|GetLocationatSplinePoint Spline PointIndex "Local"))
  (bind _index (CallFunction|GetNextSplinePoint PointIndex false))
  (bind _index_2 (CallFunction|GetNextSplinePoint PointIndex true))
  (bind _returnvalue_2 (Spline|GetNumberOfSplinePoints Spline))
  (bind _returnvalue_3 (Spline|GetLocationatSplinePoint Spline _index_2 "Local"))
  (bind _returnvalue_4 (Spline|GetLocationatSplinePoint Spline _index "Local"))
  (bind _returnvalue_5 (- _returnvalue_2 1))
  (bind _returnvalue_6 (Math|Vector|GetUnitDirection(Vector) _returnvalue _returnvalue_4))
  (bind _returnvalue_7 (Math|Vector|GetUnitDirection(Vector) _returnvalue _returnvalue_3))
  (bind _returnvalue_8 (Math|Vector|GetUnitDirection(Vector) _returnvalue_3 _returnvalue))
  (bind _returnvalue_9 (Math|Vector|GetUnitDirection(Vector) _returnvalue _returnvalue_4))
  (bind _returnvalue_10 (Math|Conversions|ToVector2D(Vector) _returnvalue_9))
  (bind _returnvalue_11 (Math|Conversions|ToVector2D(Vector) _returnvalue_8))
  (bind _returnvalue_12 (+ _returnvalue_6 _returnvalue_7))
  (bind _returnvalue_13 (Class|KismetMathLibrary|CrossProduct2D _returnvalue_10 _returnvalue_11))
  (bind _returnvalue_14 (> _returnvalue_13 0.0))
  (bind _returnvalue_15 (select _returnvalue_14 1.0 -1.0))
  (bind _returnvalue_16 (* _returnvalue_12 _returnvalue_15))
  (bind _returnvalue_17 (Math|Vector|Normalize _returnvalue_16))
  (return (select CloseMode? _returnvalue_17 (select (== PointIndex 0) (Class|SplineComponent|GetRightVectoratSplinePoint Spline 0 "Local") (select (== PointIndex _returnvalue_5) (Class|SplineComponent|GetRightVectoratSplinePoint Spline _returnvalue_5 "Local") _returnvalue_17))) _returnvalue_14))

(fn GetSplinePointHorizontalAngle
  (params (index :type Integer) (spline :type Spline%20Component%20Object%20Reference))
  (bind _returnvalue (Spline|GetLocationatSplinePoint spline index "Local"))
  (return (Class|KismetMathLibrary|DegAcos (Math|Vector2D|DotProduct(2D) (Math|Conversions|ToVector2D(Vector) (Math|Vector|GetUnitDirection(Vector) _returnvalue (Spline|GetLocationatSplinePoint spline (+ index -1) "Local"))) (Math|Conversions|ToVector2D(Vector) (Math|Vector|GetUnitDirection(Vector) _returnvalue (Spline|GetLocationatSplinePoint spline (+ index 1) "Local")))))))

(fn GetRetractPointPositionandRotation
  (params (PointIndex :type Integer) (retract :type Float%20%28double-precision%29) (spline :type Spline%20Component%20Object%20Reference) (CloseMode? :type Boolean))
  (bind _spline (LocalVariables|GetSpline))
  (bind _right_direction (CallFunction|GetSplinePointMidDirectionRight _spline PointIndex CloseMode?))
  (return (+ (* _right_direction (/ retract (Math|Trig|Cos(Degrees) (* (- 1.8e+02 (CallFunction|GetSplinePointHorizontalAngle PointIndex spline)) 0.5)))) (Spline|GetLocationatSplinePoint spline PointIndex "Local")) (Class|KismetMathLibrary|MakeRotfromYZ _right_direction (Math|Vector|MakeVector 0.0 0.0 1.0))))

(fn GetSplinePointArray
  (params (Spline :type Spline%20Component%20Object%20Reference) (CoordinateSpace :type ESplineCoordinateSpace%20Enum :default "Local") (retract :type Float%20%28double-precision%29) (ZOffset :type Float%20%28double-precision%29) (CloseMode? :type Boolean))
  (for _index (range 0 (- (Spline|GetNumberOfSplinePoints Spline) 1))
    (Development|PrintString (Utilities|String|ToString(Vector) (.Location (CallFunction|GetRetractPointPositionandRotation _index retract Spline CloseMode?))) false false)
    (Utilities|Array|Add (LocalVariables|GetPointRef) (Math|Transform|MakeTransform (+ (.Location (CallFunction|GetRetractPointPositionandRotation _index retract Spline CloseMode?)) (* (Math|Vector|GetUpVector (.Rotation (Math|Transform|BreakTransform (Spline|GetTransformatSplinePoint Spline _index CoordinateSpace false)))) ZOffset)) (.Rotation (CallFunction|GetRetractPointPositionandRotation _index retract Spline CloseMode?)) (.Scale (Math|Transform|BreakTransform (Spline|GetTransformatSplinePoint Spline _index CoordinateSpace false)))))
    (Utilities|Array|Add (LocalVariables|GetPointR) (+ (.Location (CallFunction|GetRetractPointPositionandRotation _index retract Spline CloseMode?)) (* (Math|Vector|GetUpVector (.Rotation (Math|Transform|BreakTransform (Spline|GetTransformatSplinePoint Spline _index CoordinateSpace false)))) ZOffset))))
  (return (LocalVariables|GetPointR) (LocalVariables|GetPointRef)))

(fn GetBooleMeshData
  (bind _boole_to_actor (Variables|Default|GetBoole%20To%20Actor))
  (bind _returnvalue (Transformation|GetActorTransform _boole_to_actor))
  (if (Variables|Default|GetIs%20Boole%20Prop?)
    (bind _pointarray (CallFunction|SplinePreWork))
    (bind _returnvalue_2 (DynamicMeshActor|AllocateComputeMesh))
    (bind _returnvalue_3 (Class|GeometryScriptLibraryMeshPrimitiveFunctions|AppendTriangulatedPolygon3D :TargetMesh _returnvalue_2 :PolygonVertices3D _pointarray :Debug 0))
    (bind _returnvalue_4 (Class|GeometryScriptLibraryMeshModelingFunctions|ApplyMeshLinearExtrudeFaces :TargetMesh _returnvalue_3 :Options (Utilities|Struct|MakeGeometryScriptMeshLinearExtrudeOptions (.z (Variables|Default|Gethandle)) "FixedDirection" "0.000000,0.000000,1.000000" "EntireSelection" "(GroupMode=PreserveExisting,ConstantGroup=0)" 1.0 true) :Debug 0))
    (return (Utilities|Struct|MakeST_BooleSnapData (Variables|Default|GetIs%20Boole%20Prop?) (Math|Transform|MakeTransform (Math|Transform|InverseTransformLocation _returnvalue "0, 0, 0") (Math|Transform|InverseTransformRotation _returnvalue "0, 0, 0")) _returnvalue_4 (Utilities|Array|MakeArray (Variables|Default|GetBoole%20To%20Actor))))
    (else
      (return (Utilities|Struct|MakeST_BooleSnapData false "0.000000,0.000000,0.000000|0.000000,0.000000,0.000000|1.000000,1.000000,1.000000" 0)))))

(fn GetCanbeSnapBoolePlaneData
  (return 0 0.0))