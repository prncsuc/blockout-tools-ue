(event Custom|Build
  (bind _materialconfigurationarray (Variables|Default|GetMaterialConfigurationArray))
  (bind _dynamicmeshcomponent (Variables|DynamicMeshActor|GetDynamicMeshComponent))
  (Variables|Default|SetHandle (Math|Vector|MakeVector 0.0 (.y (Variables|Default|GetHandle)) (.z (Variables|Default|GetHandle))))
  (Components|DestroyComponent (Actor|GetComponentsByClass "/Script/Engine.ChildActorComponent"))
  (DynamicMeshActor|ReleaseAllComputeMeshes)
  ;[0 0 0] Reset material
  (Utilities|Array|Clear (Variables|Default|GetMaterialConfigurationArray))
  (for _index (range 0 (- (Rendering|Material|GetNumMaterials _dynamicmeshcomponent) 1))
    (Rendering|Material|SetMaterial _dynamicmeshcomponent _index 0))
  (Class|DynamicMeshComponent|ValidateMaterialSlots _dynamicmeshcomponent true true)
  (bind _returnvalue (DynamicMeshActor|AllocateComputeMesh))
  (bind _returnvalue_2 (GeometryScript|Primitives|AppendCylinder :TargetMesh _returnvalue :Radius (.Y (Math|Vector|BreakVector (Variables|Default|GetHandle))) :Height (.Z (Math|Vector|BreakVector (Variables|Default|GetHandle))) :RadialSteps 24 :Debug 0))
  (Variables|Default|SetDynmesh _returnvalue_2)
  (Utilities|FlowControl|Sequence
    (:then_0
      (if (Variables|Default|GetHalfCircle?)
        (Class|GeometryScriptLibraryMeshBooleanFunctions|ApplyMeshPlaneCut :TargetMesh (Variables|Default|GetDynmesh) :CutFrame (Math|Transform|MakeTransform "0, 0, 0" "0.000000,0.000000,-90.000000" "1.000000,1.000000,1.000000") :Debug 0)))
    (:then_1
      (GeometryScript|UVs|ScaleMeshUVs :TargetMesh (Variables|Default|GetDynmesh) :Scale (Math|Vector2D|MakeVector2D (/ (* (.Y (Math|Vector|BreakVector (Variables|Default|GetHandle))) 3.14 2.0) 1e+02) (select (> (/ (.Z (Math|Vector|BreakVector (Variables|Default|GetHandle))) 1e+02) (/ (* (.Y (Math|Vector|BreakVector (Variables|Default|GetHandle))) 3.14 2.0) 1e+02)) (/ (.Z (Math|Vector|BreakVector (Variables|Default|GetHandle))) 1e+02) (/ (* (.Y (Math|Vector|BreakVector (Variables|Default|GetHandle))) 3.14 2.0) 1e+02))) :Debug 0)
      (Class|GeometryScriptLibraryMeshUVFunctions|TranslateMeshUVs :TargetMesh (Variables|Default|GetDynmesh) :Translation (Math|Vector2D|MakeVector2D 0.0 (Variables|Default|GetTranslation%20Y)) :Debug 0)
      (Utilities|Array|Add (Variables|Default|GetMaterialConfigurationArray) (CallFunction|CreateandSetDynamicMaterials (Variables|Default|GetMateral) (Variables|Default|GetColor%20Set) "None"))
      (Class|GeometryScriptLibraryMeshNormalsFunctions|ComputeSplitNormals :TargetMesh (Variables|Default|GetDynmesh) :SplitOptions (Utilities|Struct|MakeGeometryScriptSplitNormalsOptions true 15.0 false "(bDefaultLayer=True,ExtendedLayerIndex=0)") :Debug 0)
      (Class|DynamicMeshComponent|SetDynamicMesh (Variables|DynamicMeshActor|GetDynamicMeshComponent) (Variables|Default|GetDynmesh))
      ;[0 0 0] When the material of the component is not set, it is set to the primary material
      (for (_array_element _array_index) _materialconfigurationarray
        (if (not (Utilities|IsValid _array_element))
          (Utilities|Array|SetArrayElem _materialconfigurationarray _array_index (CallFunction|CreateandSetDynamicMaterials (Variables|Default|GetMateral) (Variables|Default|GetColor%20Set) "None"))))
      (Class|DynamicMeshComponent|ConfigureMaterialSet (Variables|DynamicMeshActor|GetDynamicMeshComponent) (Variables|Default|GetMaterialConfigurationArray)))))

(fn ConstructionScript
  (bind _returnvalue (Transformation|GetActorLocation))
  (Variables|Default|SetHandle (Math|Vector|MakeVector (.x (Variables|Default|GetHandle)) (.y (Variables|Default|GetHandle)) (select (< (.z (Variables|Default|GetHandle)) 0.0) 0.0 (.z (Variables|Default|GetHandle)))))
  (Utilities|FlowControl|Sequence
    (:then_0
      (if (Variables|Default|GetSnap？)
        (Utilities|FlowControl|Sequence
          (:then_0
            (bind (_outhit _returnvalue_2) (Collision|LineTraceForObjects _returnvalue (+ _returnvalue "0.000000,0.000000,-50.000000") (Utilities|Array|MakeArray "ObjectTypeQuery1") false 0 "None"))
            (if _returnvalue_2
              (Transformation|SetActorLocation (.Location (Collision|BreakHitResult _outhit)) false false)))
          (:then_1
            (bind (_outhit_2 _returnvalue_3) (Collision|LineTraceForObjects (+ (Transformation|GetActorLocation) (Math|Vector|MakeVector 0.0 0.0 (.z (Variables|Default|GetHandle)))) (+ (+ (Transformation|GetActorLocation) (Math|Vector|MakeVector 0.0 0.0 (.z (Variables|Default|GetHandle)))) "0.000000,0.000000,50.000000") (Utilities|Array|MakeArray "ObjectTypeQuery1") false 0 "None"))
            (if _returnvalue_3
              (Variables|Default|SetHandle (Math|Vector|MakeVector (.x (Variables|Default|GetHandle)) (.y (Variables|Default|GetHandle)) (.Z (Math|Vector|BreakVector (- (.Location (Collision|BreakHitResult _outhit_2)) (Transformation|GetActorLocation)))))))))))
    (:then_1
      (CallFunction|Build))))

(fn CreateandSetDynamicMaterials
  (params (Materal :type Material%20Interface%20Object%20Reference) (ColorSet :type ST%20Color%20Set%20V2%20Structure) (OptionalName :type Name))
  (bind (_enableset _texture _normaltex _hue _saturation _light _rough _coloroverlay _tlie _rotate) (Utilities|Struct|BreakST_ColorSetV2 ColorSet))
  (bind _returnvalue (Rendering|Material|CreateDynamicMaterialInstance (Variables|DynamicMeshActor|GetDynamicMeshComponent) (Utilities|Array|Length (Variables|Default|GetMaterialConfigurationArray)) (select (Utilities|IsValid Materal) Materal "/Game/PMB/BlockoutToolKit/Materials/Adjustable/MI_PMB_Adj__cement.MI_PMB_Adj__cement") OptionalName :!class /Script/Engine.PrimitiveComponent))
  (if _enableset
    (Rendering|Material|SetVectorParameterValue _returnvalue "Color" (Utilities|Struct|MakeLinearColor _hue _saturation _light _rough) :!class /Script/Engine.MaterialInstanceDynamic)
    (Rendering|Material|SetTextureParameterValue _returnvalue "Texture" _texture)
    (Rendering|Material|SetTextureParameterValue _returnvalue "Normal" _normaltex)
    (Rendering|Material|SetScalarParameterValue _returnvalue "Tlie" (Math|Conversions|ToFloat(Integer) _tlie) :!class /Script/Engine.MaterialInstanceDynamic)
    (Rendering|Material|SetScalarParameterValue _returnvalue "rotate" (Math|Float|MapRangeClamped (Math|Conversions|ToFloat(Integer) _rotate) 0.0 3.6e+02 0.0 1.0) :!class /Script/Engine.MaterialInstanceDynamic)
    (Rendering|Material|SetVectorParameterValue _returnvalue "ColorOverlay" _coloroverlay :!class /Script/Engine.MaterialInstanceDynamic))
  (return _returnvalue))